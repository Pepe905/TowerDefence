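; Fire tower actor that automatically shoots projectiles at Minion-tagged actors inside its range and glows to reflect day phase and threat.
; Range overlaps maintain an enemy list, with delayed removal on exit.
; Tick accumulates time to spawn projectiles aimed at the first listed enemy at a fixed interval.
; Timelines blend a dynamic material's emissive color on phase changes, plus friendly/aggressive shifts during the night phase.
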(event `ChangeTowerColor`
  (params (A :type "/Game/99_Testarea/Markus/EDayState Enum" :default "NewEnumerator0"))
  (set `self.Current Phase` A)
  (`self.DNCycleStatueGlow` A))

(event `self.ReceiveBeginPlay`
  (`KismetArrayLibrary.Array_Clear` (`self.EnemyList`))
  (`PrimitiveComponent.SetMaterial` (`self.SM_Tower`) 1 (`self.TowerGlowMatInst`))
  (bind _output_get (set `self.EmissiveColor` (struct :`G` 1.0 :`B` 0.070588 :`A` 1.0)))
  (`MaterialInstanceDynamic.SetVectorParameterValue` (`self.TowerGlowMatInst`) "EmissiveColor" _output_get))

(event `self.ReceiveTick`
  (params (DeltaSeconds :type "Float (single-precision)"))
  (if (not (`KismetArrayLibrary.Array_IsEmpty` (`self.EnemyList`)))
    (`self.DelayFire` DeltaSeconds)))

(event `self.EnemyRange.OnComponentBeginOverlap`
  (params (OverlappedComponent :type "PrimitiveComponent Object Reference") (OtherActor :type "Actor Object Reference") (OtherComp :type "PrimitiveComponent Object Reference") (OtherBodyIndex :type Integer) (bFromSweep :type Boolean) (SweepResult :type "HitResult Structure (by ref)"))
  (if (`self.ActorHasTag` OtherActor "Minion")
    (`KismetArrayLibrary.Array_Add` (`self.EnemyList`) OtherActor)
    (bind _output_get (set `self.bIsEnemyInSight` true))
    (`self.EnemyStatueGlow` _output_get)))

(event `self.EnemyRange.OnComponentEndOverlap`
  (params (OverlappedComponent :type "PrimitiveComponent Object Reference") (OtherActor :type "Actor Object Reference") (OtherComp :type "PrimitiveComponent Object Reference") (OtherBodyIndex :type Integer))
  (bind _enemylist (`self.EnemyList`))
  (if (`self.ActorHasTag` OtherActor "Minion")
    (`KismetSystemLibrary.Delay` (`self.EnemyLeftRangeDelay`))
    (`KismetArrayLibrary.Array_RemoveItem` _enemylist OtherActor)
    (if (`KismetArrayLibrary.Array_IsEmpty` _enemylist)
      (bind _output_get (set `self.bIsEnemyInSight` false))
      (`self.EnemyStatueGlow` _output_get))))

(event `DayToNight`
  ;[1 1 1] DayToNight
  (bind (_direction _transfer) (`Timeline|DayNight`)
    (:`Update`
      (`MaterialInstanceDynamic.SetVectorParameterValue` (`self.TowerGlowMatInst`) "EmissiveColor" _transfer))))

(event `GlowOnEnemy`
  (params (Condition :type Boolean))
  (if Condition
    ;[1 1 1] FriendlyToAgressive
    (bind (_direction _transfer) (`Timeline|FirendlyToAgressive`)
      (:`Update`
        (`MaterialInstanceDynamic.SetVectorParameterValue` (`self.TowerGlowMatInst`) "EmissiveColor" _transfer)))
    (else
      ;[1 1 1] AgressiveToFriendly
      (bind (_direction_2 _transfer_2) (`Timeline|AgressiveToFriendly`)
        (:`Update`
          (`MaterialInstanceDynamic.SetVectorParameterValue` (`self.TowerGlowMatInst`) "EmissiveColor" _transfer_2))))))

(event `NightToDay`
  ;[1 1 1] NightToDay
  (bind (_direction _transfer) (`Timeline|NightDay`)
    (:`Update`
      (`MaterialInstanceDynamic.SetVectorParameterValue` (`self.TowerGlowMatInst`) "EmissiveColor" _transfer))))

(fn `CreateMaterialInstance`
  (params (EmissiveColor :type "LinearColor Structure"))
  (returns (ReturnValue :type "MaterialInstanceDynamic Object Reference"))
  (bind _returnvalue (`KismetMaterialLibrary.CreateDynamicMaterialInstance` "/Game/99_Testarea/Giuseppe/Materials/MI_Statue_KnightTest.MI_Statue_KnightTest"))
  (`MaterialInstanceDynamic.SetVectorParameterValue` _returnvalue "EmissiveColor" EmissiveColor)
  (return _returnvalue))

(fn `DelayFire`
  (params (deltaTime :type "Float (double-precision)"))
  (set `self.Time` (+ deltaTime (`self.Time`)))
  (if (>= (`self.Time`) (`self.TimeBetweenShots`))
    (set `self.Time` (- (`self.Time`) (`self.TimeBetweenShots`)))
    (`self.FireEnemy`)))

(fn `DNCycleStatueGlow`
  (params (A :type "/Game/99_Testarea/Markus/EDayState Enum" :default "NewEnumerator0"))
  (if (or (`|EnumEquality` A "NewEnumerator0") (`|EnumEquality` A "NewEnumerator2"))
    (`self.NightToDay`)
    (elif (`|EnumEquality` A "NewEnumerator1")
      (`self.DayToNight`))))

(fn `EnemyStatueGlow`
  (params (bIsEnemyInSight :type Boolean))
  (if (`|EnumEquality` (`self.Current Phase`) "NewEnumerator1")
    (`self.GlowOnEnemy` bIsEnemyInSight)))

(fn `FireEnemy`
  (`self.SpawnProjectile`))

(fn `SpawnProjectile`
  (bind _returnvalue_location (`KismetMathLibrary.BreakTransform` (`SceneComponent.K2_GetComponentToWorld` (`self.SpawnProjectilePos`))))
  (bind _output (`|GetArrayItem` (`self.EnemyList`)))
  (bind _returnvalue_location_2 (`KismetMathLibrary.BreakTransform` (`SceneComponent.K2_GetComponentToWorld` (`Actor.RootComponent` _output))))
  (`/Engine/EditorBlueprintResources/StandardMacros.IsValid` _output
    (:`Is Valid`
      (bind _returnvalue (`|SpawnActorFromClass` "/Game/99_Testarea/Pepe/Projectile.Projectile_C" (`KismetMathLibrary.MakeTransform` _returnvalue_location (`KismetMathLibrary.FindLookAtRotation` _returnvalue_location _returnvalue_location_2) (0.1 0.1 0.1)) "Undefined" "OverrideRootScale" null null))
      (`/Game/99_Testarea/Pepe/Projectile.SetInit` _returnvalue "1")
      (`PrimitiveComponent.SetCollisionResponseToChannel` (`/Game/99_Testarea/Pepe/Projectile.Sphere` _returnvalue) "ECC_GameTraceChannel2" "ECR_Ignore"))))

(fn `UserConstructionScript`
  (bind _returnvalue (`self.CreateMaterialInstance` (`self.EmissiveColor`)))
  (set `self.TowerGlowMatInst` _returnvalue))