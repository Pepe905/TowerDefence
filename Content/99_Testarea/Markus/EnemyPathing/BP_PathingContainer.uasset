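; Container actor for enemy pathing that builds combined splines at runtime from a path's list of spline parts.
; AddPath spawns a static, non-ticking, collision-free spline component, stores it and fills it via CreatePath.
; CreatePath chains parts from a start location, reversing any whose end is nearer by swapping and negating tangents.
; Tangents are zeroed at part boundaries, with an extra clamped point inserted after each part.
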(fn `Add Path`
  (params (Path :type "/Game/99_Testarea/Markus/EnemyPathing/ST_Path Structure") (Location :type "Vector Structure"))
  (returns (Pathing :type "SplineComponent Object Reference"))
  (locals (counter :type Integer) (numberOfSplinePoints :type Integer) (spline :type "SplineComponent Object Reference") (pointList :type "Array of SplinePoint Structure") (currentLocation :type "Vector Structure"))
  (set `local.currentLocation` Location)
  (bind _returnvalue (`|AddComponentByClass` "/Script/Engine.SplineComponent"))
  (`SplineComponent.SetUnselectedSplineSegmentColor` _returnvalue (make `LinearColor` 0.0 1.0 0.0 1.0))
  (`SplineComponent.SetSelectedSplineSegmentColor` _returnvalue (`KismetMathLibrary.MakeColor` 1.0))
  (`SplineComponent.ClearSplinePoints` _returnvalue true)
  (`SceneComponent.SetMobility` _returnvalue "Static")
  (`BlueprintMapLibrary.Map_Add` (`self.SplineList`) (`self.Index`) _returnvalue)
  (`/Engine/EditorBlueprintResources/StandardMacros.IncrementInt` (`self.Index`)
    (:`  `
      (`self.Create Path` (`.PathParts_10_687F04E2456F2EE5AF5BE0B764942AB2` (break `/Game/99_Testarea/Markus/EnemyPathing/ST_Path` Path)) _returnvalue (`local.currentLocation`))
      (`ActorComponent.SetComponentTickEnabled` _returnvalue false)
      (`PrimitiveComponent.SetCollisionEnabled` _returnvalue "NoCollision")
      (return _returnvalue))))

(fn `AddSplinePointToList`
  (params (index :type Integer) (spline :type "SplineComponent Object Reference") (counter :type "Integer (by ref)") (splineList :type "Array of SplinePoint Structure (by ref)") (Reverse :type Boolean))
  (returns (location :type "Vector Structure"))
  (bind _splinepoint (`self.GetSplinePoint` spline index Reverse))
  (bind _structout (setmembers `SplinePoint` :`StructRef` _splinepoint :`InputKey` (`KismetMathLibrary.Conv_IntToDouble` counter)))
  (`/Engine/EditorBlueprintResources/StandardMacros.IncrementInt` counter
    (:`  `
      (`KismetArrayLibrary.Array_Add` splineList _structout)
      (return (`.Position` (break `SplinePoint` _structout))))))

(fn `CheckSplineDirection`
  (params (location :type "Vector Structure") (spline :type "SplineComponent Object Reference"))
  (returns (forward :type Boolean))
  (return (<= (`KismetMathLibrary.Vector_DistanceSquared` location (`SplineComponent.GetLocationAtSplinePoint` spline 0 "World")) (`KismetMathLibrary.Vector_DistanceSquared` location (`SplineComponent.GetLocationAtSplinePoint` spline (- (`SplineComponent.GetNumberOfSplinePoints` spline) 1) "World")))))

(fn `Create Path`
  (params (PathPartsList :type "Array of /Game/99_Testarea/Markus/EnemyPathing/BP_PathParts Object Reference") (SplinePath :type "SplineComponent Object Reference") (Location :type "Vector Structure"))
  (locals (pointList :type "Array of SplinePoint Structure") (spline :type "SplineComponent Object Reference") (currentLocation :type "Vector Structure") (numberOfSplinePoints :type Integer) (counter :type Integer))
  (set `local.currentLocation` Location)
  (for _array_element PathPartsList
    (bind _spline (`/Game/99_Testarea/Markus/EnemyPathing/BP_PathParts.Spline` _array_element))
    (set `local.spline` _spline)
    (set `local.numberOfSplinePoints` (- (`SplineComponent.GetNumberOfSplinePoints` _spline) 1))
    (if (`self.CheckSplineDirection` (`local.currentLocation`) (`local.spline`))
      (bind _location (`self.AddSplinePointToList` 0 (`local.spline`) (`local.counter`) (`local.pointList`)))
      (set `local.currentLocation` _location)
      (setmembers `SplinePoint` :`StructRef` (`|GetArrayItem` (`local.pointList`) (- (`local.counter`) 1)) :`ArriveTangent` (`KismetMathLibrary.MakeVector` 0.0) :`Type` "CurveCustomTangent")
      (for _index (range 1 (+ (`local.numberOfSplinePoints`) 1))
        (bind _location_2 (`self.AddSplinePointToList` _index (`local.spline`) (`local.counter`) (`local.pointList`)))
        (set `local.currentLocation` _location_2))
      (setmembers `SplinePoint` :`StructRef` (`|GetArrayItem` (`local.pointList`) (- (`local.counter`) 1)) :`LeaveTangent` (`KismetMathLibrary.MakeVector` 0.0) :`Type` "CurveCustomTangent")
      (`KismetArrayLibrary.Array_Add` (`local.pointList`) (make `SplinePoint` :`InputKey` (`KismetMathLibrary.Conv_IntToDouble` (`local.counter`)) :`Position` (`local.currentLocation`) :`Type` "CurveClamped"))
      (`/Engine/EditorBlueprintResources/StandardMacros.IncrementInt` (`local.counter`))
      (else
        (bind _location_3 (`self.AddSplinePointToList` (`local.numberOfSplinePoints`) (`local.spline`) (`local.counter`) (`local.pointList`) true))
        (set `local.currentLocation` _location_3)
        (setmembers `SplinePoint` :`StructRef` (`|GetArrayItem` (`local.pointList`) (- (`local.counter`) 1)) :`ArriveTangent` (`KismetMathLibrary.MakeVector` 0.0) :`Type` "CurveCustomTangent")
        (for _index_2 (range 1 (+ (`local.numberOfSplinePoints`) 1))
          (bind _location_4 (`self.AddSplinePointToList` (- (`local.numberOfSplinePoints`) _index_2) (`local.spline`) (`local.counter`) (`local.pointList`) true))
          (set `local.currentLocation` _location_4))
        (setmembers `SplinePoint` :`StructRef` (`|GetArrayItem` (`local.pointList`) (- (`local.counter`) 1)) :`LeaveTangent` (`KismetMathLibrary.MakeVector` 0.0) :`Type` "CurveCustomTangent")
        (`KismetArrayLibrary.Array_Add` (`local.pointList`) (make `SplinePoint` :`InputKey` (`KismetMathLibrary.Conv_IntToDouble` (`local.counter`)) :`Position` (`local.currentLocation`) :`Type` "CurveClamped"))
        (`/Engine/EditorBlueprintResources/StandardMacros.IncrementInt` (`local.counter`)))))
  (`SplineComponent.AddPoints` SplinePath (`local.pointList`) true))

(fn `GetSplinePoint`
  (params (spline :type "SplineComponent Object Reference") (index :type Integer) (reverse :type Boolean))
  (returns (splinePoint :type "SplinePoint Structure"))
  (locals (outSplinePoint :type "SplinePoint Structure") (worldSpace :type "ESplineCoordinateSpace Enum" :default "World"))
  (bind _returnvalue (`SplineComponent.GetSplinePointType` spline index))
  (bind _worldspace (`local.worldSpace`))
  (bind _returnvalue_2 (`SplineComponent.GetLocationAtSplinePoint` spline index _worldspace))
  (bind _returnvalue_3 (`SplineComponent.GetArriveTangentAtSplinePoint` spline index _worldspace))
  (bind _returnvalue_4 (`SplineComponent.GetLeaveTangentAtSplinePoint` spline index _worldspace))
  (set `local.worldSpace` "World")
  (if reverse
    (setmembers `SplinePoint` :`StructRef` (`local.outSplinePoint`) :`Position` _returnvalue_2 :`ArriveTangent` (* _returnvalue_4 -1.0) :`LeaveTangent` (* _returnvalue_3 -1.0) :`Rotation` (struct) :`Type` _returnvalue)
    (else
      (setmembers `SplinePoint` :`StructRef` (`local.outSplinePoint`) :`Position` _returnvalue_2 :`ArriveTangent` _returnvalue_3 :`LeaveTangent` _returnvalue_4 :`Rotation` (struct) :`Type` _returnvalue)))
  (return (`local.outSplinePoint`)))

(fn `UserConstructionScript`)