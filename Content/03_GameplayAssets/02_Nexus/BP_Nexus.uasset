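; The Nexus is an objective actor that stores mana for the player and ends the game with a "NEXUS HAS FALLEN" screen on death.
; Tick regenerates mana at intervals up to a cap, and player overlap transfers stored mana, deducting what the character takes.
; Damage events notify BP_PointSystem, found at BeginPlay and re-fetched if invalid.
; After a short delay, BeginPlay sends its location to the HUD for icon placement.
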(event `self.ReceiveBeginPlay`
  ;[1 1 1] BeginPlay & get PointSystem
  (bind _returnvalue (`GameplayStatics.GetActorOfClass` "/Game/99_Testarea/Markus/PointSystem/BP_PointSystem.BP_PointSystem_C"))
  (set `self.PointSystem` _returnvalue)
  (`KismetSystemLibrary.Delay` 0.2)
  (message `/Game/06_UI/Minimap/BPI_Minimap.UpdateIconPosition` (`PlayerController.GetHUD` (`GameplayStatics.GetPlayerController` 0)) (`KismetMathLibrary.Conv_VectorToVector2D` (`self.K2_GetActorLocation`))))

(event `/Game/99_Testarea/TonyTeststuff/BPI_ActorStateChange.Death`
  (params (selfDescruct :type Boolean))
  ;[1 1 1] Nexus destroyed
  (bind _returnvalue (`GameplayStatics.GetActorOfClass` "/MoveIt/Example/BP_MoveIt_ExampleCharacter.BP_MoveIt_ExampleCharacter_C"))
  (`/Game/06_UI/WB_HUD.GameOver` (`/MoveIt/Example/BP_MoveIt_ExampleCharacter.DemoWidget` _returnvalue) "NEXUS HAS FALLEN"))

(event `/Game/99_Testarea/TonyTeststuff/BPI_ActorStateChange.DmgTaken`
  ;[1 1 1] Message Pointsystem on Damage
  (`/Engine/EditorBlueprintResources/StandardMacros.IsValid` (`self.PointSystem`)
    (:`Is Valid`
      _)
    (:`Is Not Valid`
      (bind _returnvalue (`GameplayStatics.GetActorOfClass` "/Game/99_Testarea/Markus/PointSystem/BP_PointSystem.BP_PointSystem_C"))
      (set `self.PointSystem` _returnvalue)))
  (`/Game/99_Testarea/Markus/PointSystem/BP_PointSystem.NexusTakeDmg` (`self.PointSystem`)))

(event `self.ReceiveTick`
  (params (DeltaSeconds :type "Float (single-precision)"))
  ;[1 1 1] AddMana in Interval till ManaMax is met
  (bind _output_get (set `self.ManaGainTimer` (+ DeltaSeconds (`self.ManaGainTimer`))))
  (if (>= _output_get (`self.ManaGainIntervall`))
    (`self.ManaGain` (`self.ManaIncrease`))))

(event `self.ReceiveActorBeginOverlap`
  (params (OtherActor :type "Actor Object Reference"))
  (if (== (`GameplayStatics.GetObjectClass` OtherActor) "/MoveIt/Example/BP_MoveIt_ExampleCharacter.BP_MoveIt_ExampleCharacter_C")
    (bind _asbp_move_it_example_character (cast `/MoveIt/Example/BP_MoveIt_ExampleCharacter` OtherActor))
    (bind _manadrained (`/MoveIt/Example/BP_MoveIt_ExampleCharacter.ReceivaManaFromNexus` _asbp_move_it_example_character (`self.ManaCurrent`)))
    (set `self.ManaCurrent` (- (`self.ManaCurrent`) _manadrained))))

(fn `ManaGain`
  (params (ManaIncrease :type "Float (double-precision)"))
  (if (< (`self.ManaCurrent`) (`self.ManaMax`))
    (set `self.ManaCurrent` (+ (`self.ManaCurrent`) ManaIncrease))
    (set `self.ManaGainTimer` 0.0)
    (else
      (set `self.ManaCurrent` (`self.ManaMax`)))))

(fn `UserConstructionScript`)