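; Tower defence game mode Blueprint that registers the level's BP_Grid actors at BeginPlay and serves as their lookup point.
; It stores each grid in a map under a numbered "Grid" name and caches the first one found as the default Grid.
; GetGrid and GetAllGrids expose these; the trailing delay triggers nothing, and the debug print and HUD creation nodes are disconnected.
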(event `self.ReceiveBeginPlay`
  (`|ExecutionSequence`
    (:`then_0`
      (bind _outactors (`GameplayStatics.GetAllActorsOfClass` "/Game/99_Testarea/Giuseppe/Blueprints/BP_Grid.BP_Grid_C"))
      (for _array_element _outactors
        (set `self.Grid` (`|GetArrayItem` _outactors))
        (`BlueprintMapLibrary.Map_Add` (`self.Grid in World`) (`KismetSystemLibrary.MakeLiteralString` (`KismetStringLibrary.Concat_StrStr` "Grid" " " (`KismetStringLibrary.Conv_IntToString` (`self.GridNumber`)))) _array_element)
        (set `self.GridNumber` (+ (`self.GridNumber`) 1))))
    (:`then_1`
      (`KismetSystemLibrary.Delay` 0.2))))

(fn `GetAllGrids`
  (returns (`Grid in World` :type "Map of String to /Game/99_Testarea/Giuseppe/Blueprints/BP_Grid Object Reference"))
  (return (`self.Grid in World`)))

(fn `GetGrid`
  (returns (Grid :type "/Game/99_Testarea/Giuseppe/Blueprints/BP_Grid Object Reference"))
  (return (`self.Grid`)))

(fn `UserConstructionScript`)