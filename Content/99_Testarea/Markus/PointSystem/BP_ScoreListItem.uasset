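; BP_ScoreListItem holds one ranked entry for a score list.
; SetData takes a rank and a data struct with ID, name, score, kills, rounds and time, and routes them through a collapsed graph of to-text conversions.
; SetNemberData then passes the results to SetNembersData, which stores each in its matching member variable.
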(fn `SetData`
  (params (rank :type Integer) (data :type "ST_ScoreData Structure"))
  (bind (_id _name _score _kills _rounds _time) (break `ST_ScoreData` data))
  (`self.SetNemberData` (`KismetTextLibrary.Conv_IntToText` _id) (`KismetTextLibrary.Conv_StringToText` _name) (`KismetTextLibrary.Conv_IntToText` _score) (`KismetTextLibrary.Conv_IntToText` _kills) (`KismetTextLibrary.Conv_IntToText` _rounds) (`KismetTextLibrary.Conv_StringToText` _time) (`KismetTextLibrary.Conv_IntToText` rank)))

(fn `SetNemberData`
  (params (id :type Text) (name :type Text) (score :type Text) (kills :type Text) (rounds :type Text) (time :type Text) (rank :type Text))
  (set `self.ID` id)
  (set `self.Name` name)
  (set `self.Score` score)
  (set `self.Kills` kills)
  (set `self.Rounds` rounds)
  (set `self.Rank` rank)
  (set `self.Time` time))