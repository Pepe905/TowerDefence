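; BP_TestTower is a test tower that shoots projectiles at enemies.
; Each tick it rotates SpawnProjectilePos toward the first BP_EnemyTest found in the world, regardless of range.
; An actor tagged "Minion" entering EnemyRange triggers FireEvent, spawning one scaled-down projectile along that aim, with no repeat fire.
; It caches BP_SpawnManager on BeginPlay but does not use it in these graphs.
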(event `self.ReceiveBeginPlay`
  (bind _returnvalue (`GameplayStatics.GetActorOfClass` "/Game/TonyTeststuff/BP_SpawnManager.BP_SpawnManager_C"))
  (set `self.SpawnManager` _returnvalue))

(event `self.ReceiveTick`
  (params (DeltaSeconds :type "Float (single-precision)"))
  (bind _returnvalue (`GameplayStatics.GetActorOfClass` "/Game/TonyTeststuff/BP_EnemyTest.BP_EnemyTest_C"))
  (`/Engine/EditorBlueprintResources/StandardMacros.IsValid` _returnvalue
    (:`Is Valid`
      (`SceneComponent.K2_SetWorldRotation` (`self.SpawnProjectilePos`) (`KismetMathLibrary.FindLookAtRotation` (`SceneComponent.K2_GetComponentLocation` (`self.SpawnProjectilePos`)) (`self.K2_GetActorLocation` _returnvalue)) false false))))

(event `self.EnemyRange.OnComponentBeginOverlap`
  (params (OverlappedComponent :type "PrimitiveComponent Object Reference") (OtherActor :type "Actor Object Reference") (OtherComp :type "PrimitiveComponent Object Reference") (OtherBodyIndex :type Integer) (bFromSweep :type Boolean) (SweepResult :type "HitResult Structure (by ref)"))
  (if (`self.ActorHasTag` OtherActor "Minion")
    (`self.FireEvent`)))

(event `FireEvent`
  (bind (_returnvalue_location _returnvalue_rotation) (`KismetMathLibrary.BreakTransform` (`SceneComponent.K2_GetComponentToWorld` (`self.SpawnProjectilePos`))))
  (`|SpawnActorFromClass` "/Game/Pepe/Projectile.Projectile_C" (`KismetMathLibrary.MakeTransform` _returnvalue_location _returnvalue_rotation (0.1 0.1 0.1)) "Undefined" "OverrideRootScale" null null))

(fn `UserConstructionScript`)