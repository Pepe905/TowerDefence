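; BP_NiagaraTowerTest is a test tower Blueprint that plays a Niagara-driven upgrade transition.
; UpgradeTower runs once, loads the next tower's row from DT_TowerDetails, shows the Niagara component, then calls Upgrade and ChangeTowerType.
; Upgrade runs a timeline that feeds one animation value to both the tower mesh materials and the Niagara effect, hiding the mesh partway through.
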(event `self.ReceiveBeginPlay`
  (`parent.ReceiveBeginPlay`))

(event `Upgrade`
  (bind (_direction _newtrack_0) (`Timeline|Timeline`)
    (:`Update`
      (`MeshComponent.SetScalarParameterValueOnMaterials` (`self.SM_Tower`) "Animation" _newtrack_0)
      (`NiagaraComponent.SetNiagaraVariableFloat` (`self.Niagara1`) "CustomAnimation" _newtrack_0)
      (if (>= _newtrack_0 0.23)
        (`SceneComponent.SetVisibility` (`self.SM_Tower`) false false)))))

(fn `UpgradeTower`
  (returns (`Succesful Upgrade?` :type Boolean))
  (if (`self.IsUpgraded?`)
    (return false)
    (else
      (set `self.IsUpgraded?` true)
      (bind _returnvalue (`|GetDataTableRow` "/Game/99_Testarea/Giuseppe/Blueprints/Tower/DT_TowerDetails.DT_TowerDetails" (`.UpgradeToTower_41_9612E6914B6A4BB3EF254280ACFBFFA4` (break `/Game/99_Testarea/Giuseppe/Blueprints/Tower/ST_TowerDetails` (`self.Tower details`))))
        (:`then`
          (set `self.Tower details` _returnvalue)
          (`SceneComponent.SetVisibility` (`self.Niagara1`) true false)
          (`self.Upgrade`)
          (`self.ChangeTowerType`)
          (set `self.SuccessfullUpgrade` true)
          (return true))))))

(fn `UserConstructionScript`
  (`parent.UserConstructionScript`))