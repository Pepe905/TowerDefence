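; Card manager actor that rolls random card drops at a world location and pools the BP_Card actors used for them.
; A random percentage is tested against cumulative DropChance values from DT_Cards to choose the card ID.
; SpawnCard moves a pooled card from passive to active and places it, while DespawnCard returns it.
; The pool fills in batches on BeginPlay and when empty, though an empty-pool request spawns no card.
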(event `self.ReceiveBeginPlay`
  (`self.IncreaseCardPool`))

(fn `CardDropCalculation`
  (params (WorldLocation :type "Vector Structure"))
  (locals (RandomPercentageValue :type "Float (double-precision)") (CurrentStartRandom :type "Float (double-precision)") (TmpCardRowName :type Name))
  (set `local.RandomPercentageValue` (`KismetMathLibrary.RandomFloatInRange` 0.0 100.0))
  (bind _outrownames (`DataTableFunctionLibrary.GetDataTableRowNames` "/Game/06_UI/01_Cards/DT_Cards.DT_Cards"))
  (for _array_element _outrownames
    (bind _returnvalue (`|GetDataTableRow` "/Game/06_UI/01_Cards/DT_Cards.DT_Cards" _array_element)
      (:`then`
        (bind ((`DropChance_43_10AAC9D343125BFA8F202BBB05EFE01D` _dropchance)) (break `/Game/06_UI/01_Cards/ST_Cards` _returnvalue))
        (if (>= (+ _dropchance (`local.CurrentStartRandom`)) (`local.RandomPercentageValue`))
          (`self.SpawnCard` WorldLocation _array_element)
          (break)
          (else
            (set `local.CurrentStartRandom` (+ _dropchance (`local.CurrentStartRandom`)))))))))

(fn `DespawnCard`
  (params (Card :type "/Game/06_UI/01_Cards/BP_Card Object Reference"))
  (`KismetArrayLibrary.Array_Remove` (`self.CardPoolACTIVE`) (`KismetArrayLibrary.Array_Find` (`self.CardPoolACTIVE`) Card))
  (`KismetArrayLibrary.Array_Add` (`self.CardPoolPASSIVE`) Card))

(fn `IncreaseCardPool`
  (for _ (range 50)
    (bind _returnvalue (`|SpawnActorFromClass` "/Game/06_UI/01_Cards/BP_Card.BP_Card_C" (`self.GetTransform` self) "AdjustIfPossibleButAlwaysSpawn" "OverrideRootScale" null null))
    (`/Game/06_UI/01_Cards/BP_Card.InitCard` _returnvalue)
    (set `/Game/06_UI/01_Cards/BP_Card.CardManager` self _returnvalue)
    (`KismetArrayLibrary.Array_Add` (`self.CardPoolPASSIVE`) _returnvalue)))

(fn `SpawnCard`
  (params (WorldLocation :type "Vector Structure") (CardID :type Name))
  (locals (TmpCard :type "/Game/06_UI/01_Cards/BP_Card Object Reference"))
  (bind _output (`|GetArrayItem` (`self.CardPoolPASSIVE`)))
  (if (`KismetSystemLibrary.IsValid` _output)
    (set `local.TmpCard` _output)
    (`KismetArrayLibrary.Array_Remove` (`self.CardPoolPASSIVE`))
    (`KismetArrayLibrary.Array_Add` (`self.CardPoolACTIVE`) (`local.TmpCard`))
    (`SceneComponent.K2_SetWorldLocation` (`/Game/06_UI/01_Cards/BP_Card.DefaultSceneRoot` (`local.TmpCard`)) WorldLocation false false)
    (`/Game/06_UI/01_Cards/BP_Card.SpawnCard` (`local.TmpCard`) CardID)
    (else
      (`self.IncreaseCardPool`))))

(fn `UserConstructionScript`)