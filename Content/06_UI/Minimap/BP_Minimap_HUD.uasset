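; BP_Minimap_HUD feeds the player's position to the minimap and relays icon position updates to the demo widget.
; On BeginPlay it caches DemoWidget from the BP_MoveIt_ExampleCharacter in the level.
; Every Tick it writes the player character's location to the "Player Location" vector in the MP_Minimap material parameter collection.
; UpdateIconPosition forwards a given position to the widget's UpdateIconLocation when the widget is valid.
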(event `self.ReceiveBeginPlay`
  (bind _returnvalue (`GameplayStatics.GetActorOfClass` "/MoveIt/Example/BP_MoveIt_ExampleCharacter.BP_MoveIt_ExampleCharacter_C"))
  (set `self.Demo Widget` (`/MoveIt/Example/BP_MoveIt_ExampleCharacter.DemoWidget` _returnvalue)))

(event `self.ReceiveTick`
  (params (DeltaSeconds :type "Float (single-precision)"))
  (`KismetMaterialLibrary.SetVectorParameterValue` "/Game/06_UI/Minimap/MP_Minimap.MP_Minimap" "Player Location" (`KismetMathLibrary.Conv_VectorToLinearColor` (`self.K2_GetActorLocation` (`GameplayStatics.GetPlayerCharacter` 0)))))

(event `/Game/06_UI/Minimap/BPI_Minimap.UpdateIconPosition`
  (params (position :type "Vector2D Structure"))
  (bind _demo_widget (`self.Demo Widget`)
    (:`then`
      (`/Game/06_UI/WB_HUD.UpdateIconLocation` _demo_widget position))
    (:`else`)))

(fn `UserConstructionScript`)