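; Spawn manager that runs enemy waves across the active portals and keeps an object pool of BP_EnemyTest actors.
; The pool is pre-spawned in batches at BeginPlay and whenever the passive list runs out.
; Each wave raises the spawn count, moves pooled enemies to the active list and hands them to each portal, adjusted by its modifier.
; Despawned enemies return to the pool, and an empty active list starts the day phase when checked.
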(event `self.ReceiveBeginPlay`
  (`self.IncreaseEnemyPool`))

(event `NextWave`
  ;[1 1 1] Call Spawn of next wave on all active portals
  (`/Engine/EditorBlueprintResources/StandardMacros.IncrementInt` (`self.WaveCounter`)
    (:`  `
      (`/Engine/EditorBlueprintResources/StandardMacros.IncrementInt` (`self.EnemyToSpawn`)
        (:`  `
          (for _array_element (`self.PortalActive`)
            (set `self.PortalSpawning` _array_element)
            (`self.SpawnEnemiesAtPortal`))
          (set `self.EnemiesKilled` 0)
          (`self.UpdateEnemyLeft`))))))

(fn `CheckEnemiesLeft`
  (`self.UpdateEnemyLeft`)
  (if (== (`self.EnemyLeft`) 0)
    (`/Game/99_Testarea/Markus/BP_DayNightCycle.StartDayPhase` (`self.DayNightCycle`))))

(fn `DespawnEnemies`
  (params (Enemy :type "/Game/04_Characters/02_Enemies/BP_EnemyTest Object Reference"))
  (locals (EnemyTmp :type "/Game/04_Characters/02_Enemies/BP_EnemyTest Object Reference"))
  (`KismetArrayLibrary.Array_Remove` (`self.EnemyPoolACTIVE`) (`KismetArrayLibrary.Array_Find` (`self.EnemyPoolACTIVE`) Enemy))
  (`KismetArrayLibrary.Array_Add` (`self.EnemyPoolPASSIVE`) Enemy))

(fn `IncreaseEnemyPool`
  (for _ (range 50)
    (bind _returnvalue (`|SpawnActorFromClass` "/Game/04_Characters/02_Enemies/BP_EnemyTest.BP_EnemyTest_C" (`self.GetTransform` self) "AdjustIfPossibleButAlwaysSpawn" "OverrideRootScale" null null))
    (`KismetArrayLibrary.Array_Add` (`self.EnemyPoolPASSIVE`) _returnvalue)))

(fn `SpawnEnemiesAtPortal`
  (locals (EnemyTmp :type "/Game/04_Characters/02_Enemies/BP_EnemyTest Object Reference") (EnemyToSpawnHere :type "Array of /Game/04_Characters/02_Enemies/BP_EnemyTest Object Reference"))
  (bind _output (`|GetArrayItem` (`self.EnemyPoolPASSIVE`)))
  (for _ (range (+ (+ (`self.EnemyToSpawn`) (`/Game/03_GameplayAssets/05_Portals/BP_Portal.SpawnCountModifier` (`self.PortalSpawning`))) 1))
    (if (`KismetSystemLibrary.IsValid` _output)
      (set `local.EnemyTmp` _output)
      (`KismetArrayLibrary.Array_Remove` (`self.EnemyPoolPASSIVE`))
      (`KismetArrayLibrary.Array_Add` (`self.EnemyPoolACTIVE`) (`local.EnemyTmp`))
      (`KismetArrayLibrary.Array_Add` (`/Game/03_GameplayAssets/05_Portals/BP_Portal.EnemiesToSpawn` (`self.PortalSpawning`)) (`local.EnemyTmp`))
      (else
        (`self.IncreaseEnemyPool`))))
  (`/Game/03_GameplayAssets/05_Portals/BP_Portal.SpawnEnemies` (`self.PortalSpawning`)))

(fn `UpdateEnemyLeft`
  (set `self.EnemyLeft` (`KismetArrayLibrary.Array_Length` (`self.EnemyPoolACTIVE`))))

(fn `UpdateKilledEnemies`
  (`/Engine/EditorBlueprintResources/StandardMacros.IncrementInt` (`self.EnemiesKilled`)
    (:`  `
      (`/Engine/EditorBlueprintResources/StandardMacros.IncrementInt` (`self.GlobalEnemyCounter`)
        (:`  `
          (`self.UpdateEnemyLeft`))))))

(fn `UserConstructionScript`)