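; BP_Door is a door the player opens on hit or overlap, unless the day/night cycle is in one excluded state.
; The first door each round is free; further doors cost player mana, with a widget message when short.
; Opening increments the spawn manager's door count, activates linked portals, frees linked paths and destroys the door.
; In one specific day state, opening also starts the day/night cycle.
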(event `self.ReceiveBeginPlay`
  ;[1 1 1] On BeginPlay, get Player & DayNightCycle
  (bind _returnvalue (`GameplayStatics.GetActorOfClass` "/MoveIt/Example/BP_MoveIt_ExampleCharacter.BP_MoveIt_ExampleCharacter_C"))
  (set `self.Player` _returnvalue)
  (bind _returnvalue_2 (`GameplayStatics.GetActorOfClass` "/Game/99_Testarea/Markus/BP_DayNightCycle.BP_DayNightCycle_C"))
  (set `self.DayNightCycle` _returnvalue_2)
  (bind _returnvalue_3 (`GameplayStatics.GetActorOfClass` "/Game/03_GameplayAssets/05_Portals/BP_EnemySpawnManager.BP_EnemySpawnManager_C"))
  (set `self.SpawnManager` _returnvalue_3))

(event `self.ReceiveHit`
  (params (MyComp :type "PrimitiveComponent Object Reference") (Other :type "Actor Object Reference") (OtherComp :type "PrimitiveComponent Object Reference") (bSelfMoved :type Boolean) (HitLocation :type "Vector Structure") (HitNormal :type "Vector Structure") (NormalImpulse :type "Vector Structure") (Hit :type "HitResult Structure (by ref)"))
  ;[1 1 1] On Open, Activate all connected Portals & Destroy self afterwards
  (if (== (stale `self.ReceiveActorBeginOverlap` OtherActor) (`self.Player`)) :!label _label
    (if (`|EnumInequality` (`/Game/99_Testarea/Markus/BP_DayNightCycle.DayState` (`self.DayNightCycle`)) "NewEnumerator1")
      (bind _canopendoor (`self.CanOpenDoor?`))
      (if _canopendoor
        (`/Engine/EditorBlueprintResources/StandardMacros.IncrementInt` (`/Game/03_GameplayAssets/05_Portals/BP_EnemySpawnManager.DoorCount` (`self.SpawnManager`))
          (:`  `
            (`SceneComponent.SetVisibility` (`self.Cube`) false false)
            (for _array_element (`self.Portal`)
              (`/Game/03_GameplayAssets/05_Portals/BP_Portal.Activation` _array_element))
            (if (`|EnumEquality` (`/Game/99_Testarea/Markus/BP_DayNightCycle.DayState` (`self.DayNightCycle`)) "NewEnumerator2")
              (`/Game/99_Testarea/Markus/BP_DayNightCycle.StartDayNigthCyle` (`self.DayNightCycle`)))
            (for _array_element_2 (`self.Paths`)
              (set `/Game/99_Testarea/Markus/EnemyPathing/BP_PathParts.IsFree` true _array_element_2))
            (`self.K2_DestroyActor`)))))))

(event `self.ReceiveActorBeginOverlap`
  (params (OtherActor :type "Actor Object Reference"))
  ;[1 1 1] On Open, Activate all connected Portals & Destroy self afterwards
  (`KismetSystemLibrary.PrintString` "door overlap")
  (goto _label))

(fn `CanOpenDoor?`
  (returns (CanOpenDoor :type Boolean))
  (locals (CanOpen :type Boolean))
  (if (`/Game/99_Testarea/Markus/BP_DayNightCycle.DoorOpenedThisRound?` (`self.DayNightCycle`))
    (bind _output_get (set `local.CanOpen` (>= (`/MoveIt/Example/BP_MoveIt_ExampleCharacter.ManaCurrent` (`self.Player`)) 10.0)))
    (if _output_get
      (set `/MoveIt/Example/BP_MoveIt_ExampleCharacter.ManaCurrent` (- (`/MoveIt/Example/BP_MoveIt_ExampleCharacter.ManaCurrent` (`self.Player`)) 10.0) (`self.Player`))
      (else
        (`/Game/06_UI/WB_HUD.Message_CannotUseCard` (`/MoveIt/Example/BP_MoveIt_ExampleCharacter.DemoWidget` (`self.Player`)) "CANT OPEN DOOR - NOT ENOUGH MANA")))
    (return (`local.CanOpen`))
    (else
      (bind _output_get_2 (set `/Game/99_Testarea/Markus/BP_DayNightCycle.DoorOpenedThisRound?` true (`self.DayNightCycle`)))
      (return _output_get_2))))

(fn `UserConstructionScript`)