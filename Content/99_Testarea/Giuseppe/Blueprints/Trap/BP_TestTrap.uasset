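; Deprecated test trap Blueprint whose Tick, BeginPlay and overlap events are empty, leaving its main logic disconnected.
; The unwired logic configures mesh, fire rate and projectile from DT_TowerDetails, then box-scans for a target and applies projectile data on a timer.
; It can also send overlapped enemies down one of two dodge-lane splines.
; An older, also unwired overlap path damages "Minion" actors through AC_Healthmanagement with a looped-back cooldown.
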(event `self.Range.OnComponentBeginOverlap`
  (params (OverlappedComponent :type "PrimitiveComponent Object Reference") (OtherActor :type "Actor Object Reference") (OtherComp :type "PrimitiveComponent Object Reference") (OtherBodyIndex :type Integer) (bFromSweep :type Boolean) (SweepResult :type "HitResult Structure (by ref)"))
  ;[0.9133 1 0] Deprecated
)

(event `ResetCooldown`
  ;[0.9133 1 0] Deprecated
  (set `self.bShouldWait` false)
  (`/Engine/EditorBlueprintResources/StandardMacros.DoOnce` false :!via `Reset`
    (:`Completed`
      (`self.DamageEnemy`)
      (set `self.bShouldWait` true)
      (`KismetSystemLibrary.K2_SetTimerDelegate` (delegate `ResetCooldown`) 1.0))))

(event `self.Range.OnComponentEndOverlap`
  (params (OverlappedComponent :type "PrimitiveComponent Object Reference") (OtherActor :type "Actor Object Reference") (OtherComp :type "PrimitiveComponent Object Reference") (OtherBodyIndex :type Integer))
  ;[0.9133 1 0] Deprecated
)

(event `DamageEnemy`
  (`/Game/99_Testarea/TonyTeststuff/AC_Healthmanagement.TakeDamage` (`self.HealthManager`) (`self.TrapDamage`)))

(event `self.ReceiveTick`
  (params (DeltaSeconds :type "Float (single-precision)")))

(event `self.ReceiveBeginPlay`)

(fn `ChangeTrapType`
  (bind _skeletalmesh_trap (`self.SkeletalMesh_Trap`))
  (bind ((`FireRate_31_8BDF542148809F4CB7D434BF6645CB0D` _firerate) (`BulletID_34_C53CF9C541DC7EE7A332B78111B69322` _bulletid) (`StaticMesh_44_252780A941DD4F1B936A538182551656` _staticmesh) (`WeaponMesh_69_B86B4FC14D01DB46D5762081EDE72EE2` _weaponmesh) (`PlacementSFX_72_A8AC0E4A4CE5346A1BEB268EC2F0FE82` _placementsfx) (`PlacementVFX_73_A1B7A7D549AB611983A716A928AA5BC6` _placementvfx) (`TrapPreviewVFX_59_0B0E738D464F396B4D6065B084073C2E` _trappreviewvfx) (`UpgradeSFX_76_1FFA35BA472949A6E2441997A71AB7E8` _upgradesfx) (`UpgradeVFX_77_5E8852124043E12371C02D81B660325E` _upgradevfx) (`UseDodgePath_79_1B19ADB443F8382545B1F4B0B41411D2` _usedodgepath) (`DodgePathIndex_83_2AD35DE44EFA80220EA459A7F2FEA0B5` _dodgepathindex) (`WeaponMat_87_0CBAEC694EDB84DF418111AC05E2A7C8` _weaponmat) (`SM_Trap_94_0CDB2BEB4594999B29680FA785E4DD16` _sm_trap) (`TrapAB_97_391446D94F9BCBD3A01F33910C792D47` _trapab)) (break `/Game/99_Testarea/Giuseppe/Blueprints/Tower/ST_TowerDetails` (`self.Out Row`)))
  (set `self.Time Between Shots` _firerate)
  (set `self.Projetile ID` _bulletid)
  (set `self.UseDogeLane` _usedodgepath)
  (set `self.DogeLaneIndex` _dodgepathindex)
  (bind _output_get (set `self.SM_Trap` _sm_trap))
  (`SkeletalMeshComponent.SetSkeletalMeshAsset` _skeletalmesh_trap _output_get)
  (`SkeletalMeshComponent.SetAnimInstanceClass` _skeletalmesh_trap (`GameplayStatics.GetObjectClass` _trapab)))

(fn `DamageTarget`
  (bind _targetedenemy (`self.TargetedEnemy`))
  (`/Engine/EditorBlueprintResources/StandardMacros.IsValid` (`self.TargetedEnemy`)
    (:`Is Valid`
      (bind _projectiledata (`/Game/99_Testarea/Markus/ProjectileData/BP_ProjectileDataHandle.GetProjectileData` (`self.Projetile ID`)))
      (set `self.Projectile Data` _projectiledata)
      (`/Game/99_Testarea/Markus/ProjectileData/BP_ProjectileDataHandle.HandleProjectileData` (`self.Projectile Data`) _targetedenemy)
      (`/Game/99_Testarea/Markus/ProjectileData/BP_ProjectileDataHandle.PlayImpactEffectAtActorPosition` (`self.Projectile Data`) _targetedenemy)
      (set `self.TargetedEnemy` null)
      (set `self.ReadyToFire` false))))

(fn `DelayDamage`
  (params (DeltaTime :type "Float (double-precision)")))

(fn `FindEnemy`
  (bind _outactors (`KismetSystemLibrary.BoxOverlapActors` (`self.K2_GetActorLocation` self) (180.0 180.0 180.0) (`|MakeArray` "ObjectTypeQuery9" :!type "EObjectTypeQuery Enum")))
  (bind _output_get (set `self.EnemiesOverlapping` _outactors))
  (bind _output_get_2 (set `self.TargetedEnemy` (`|GetArrayItem` _output_get))))

(fn `ReadyToShoot`
  (params (DeltaTime :type "Float (double-precision)"))
  (set `self.Time` (+ DeltaTime (`self.Time`)))
  (if (>= (`self.Time`) (`self.Time Between Shots`))
    (set `self.Time` (- (`self.Time`) (`self.Time Between Shots`)))
    (set `self.ReadyToFire` true)))

(fn `SetDogeLaneOnEnemies`
  (bind _enemiesoverlapping (`self.EnemiesOverlapping`))
  (if (and (`self.UseDogeLane`) (not (`KismetArrayLibrary.Array_IsEmpty` _enemiesoverlapping)))
    (for _array_element _enemiesoverlapping
      (`/Game/04_Characters/02_Enemies/BP_EnemyTest.StartDogePath` (cast `/Game/04_Characters/02_Enemies/BP_EnemyTest` _array_element :!pure true) (`|GetArrayItem` (`self.DogeLane`) (`self.DogeLaneIndex`)) self))))

(fn `SetTrapType`
  (params (TrapID :type Name))
  (bind _returnvalue (`|GetDataTableRow` "/Game/99_Testarea/Giuseppe/Blueprints/Tower/DT_TowerDetails.DT_TowerDetails" TrapID)
    (:`then`
      (set `self.Out Row` _returnvalue)
      (`self.ChangeTrapType`)
      (return))))

(fn `UserConstructionScript`)