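; Day/night cycle manager that alternates a timed building day with a night wave phase.
; Tick runs only by day, counting down to SkipDayPhase, which starts the next, optionally elite or final, spawn-manager wave.
; StartDayPhase declares victory after the final wave, otherwise respawns artefacts and restarts the timer.
; Transitions switch sound, barriers, lighting and building mode, and notify HUD, grid and traps; construction registers it with the spawn manager.
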(event `self.ReceiveBeginPlay`
  (`self.SetActorTickEnabled` false)
  (bind _returnvalue (`GameplayStatics.GetActorOfClass` "/MoveIt/Example/BP_MoveIt_ExampleCharacter.BP_MoveIt_ExampleCharacter_C"))
  (set `self.Player` _returnvalue)
  (set `self.DayTimeLeft` (`KismetMathLibrary.FTrunc` (`self.MaxDayTime`)))
  (bind _returnvalue_2 (`GameplayStatics.SpawnSound2D` "/Game/07_Audio/BackgroundMusic/DayPhase/DayPhase.DayPhase" 1.0 1.0 0.0 null false false))
  (bind _output_get (set `self.DaySoundObject` _returnvalue_2))
  (`ActorComponent.SetActive` _output_get false false)
  (bind _returnvalue_3 (`GameplayStatics.SpawnSound2D` "/Game/07_Audio/BackgroundMusic/NightPhase/NightPhase.NightPhase" 1.0 1.0 0.0 null false false))
  (bind _output_get_2 (set `self.NightSoundObject` _returnvalue_3))
  (`ActorComponent.SetActive` _output_get_2 false false))

(event `self.ReceiveTick`
  (params (DeltaSeconds :type "Float (single-precision)"))
  (if (`|EnumEquality` (`self.DayState`) "NewEnumerator0")
    (set `self.DayTime` (+ (`self.DayTime`) DeltaSeconds))
    (set `self.DayTimeLeft` (`KismetMathLibrary.FTrunc` (- (`self.MaxDayTime`) (`self.DayTime`))))
    (if (>= (`self.DayTime`) (`self.MaxDayTime`))
      (`self.SkipDayPhase` false))))

(fn `SetLight`
  (params (LightConfig :type "/Game/99_Testarea/Markus/ST_LightingConfig Structure"))
  (`LightComponent.SetIntensity` (`Light.LightComponent` LightConfig_Light_28_5268DDAE4D9206514ABB339AC7CD93B2) LightConfig_LightIntensity_14_22992E934DED4E689933F69E1D86A7E8)
  (`LightComponent.SetTemperature` (`Light.LightComponent` LightConfig_Light_28_5268DDAE4D9206514ABB339AC7CD93B2) LightConfig_LightTemperature_31_6519342147DFF47BDCB29989BA2A284D))

(fn `SkipDayPhase`
  (params (`EliteRound?` :type Boolean) (`FinalWave?` :type Boolean))
  (`ActorComponent.SetActive` (`self.NightSoundObject`) true false)
  (`ActorComponent.SetActive` (`self.DaySoundObject`) false false)
  (`/Game/03_GameplayAssets/03_Artefacts/BP_ArtefactSpawner.ActivateBarriers` (`self.ArtefactManager`))
  (set `self.DoorOpenedThisRound?` false)
  (if (`|EnumEquality` (`self.DayState`) "NewEnumerator0")
    (set `self.DayState` "NewEnumerator1")
    (`self.SetLight` (`self.NightLight`))
    (set `self.DayTimeLeft` 0)
    (`self.SetActorTickEnabled` false)
    (`/Game/03_GameplayAssets/05_Portals/BP_EnemySpawnManager.NextWave` (`self.SpawnManager`) `EliteRound?`)
    (if `EliteRound?`
      (`/Game/06_UI/WB_HUD.CollectArtefact` (`self.HUD`))
      (if `FinalWave?`
        (set `self.FinalWave?` true)
        (`/Game/06_UI/WB_HUD.StartFinalWave` (`self.HUD`))
        (else
          (`/Game/06_UI/WB_HUD.StartNightphase` (`self.HUD`) :!label _label)))
      (else
        (goto _label)))
    (`/MoveIt/Example/BP_MoveIt_ExampleCharacter.Stop Building Mode` (`self.Player`))
    (bind _returnvalue (`GameplayStatics.GetActorOfClass` "/Game/99_Testarea/Giuseppe/Blueprints/BP_Grid.BP_Grid_C"))
    (bind _output_get (set `self.Grid` _returnvalue))
    (`/Game/99_Testarea/Giuseppe/Blueprints/BP_Grid.CallCycleChange` _output_get (`self.DayState`))
    (bind _outactors (`GameplayStatics.GetAllActorsOfClass` "/Game/99_Testarea/Giuseppe/Blueprints/Trap/BP_TestTrap.BP_TestTrap_C"))
    (for _array_element _outactors
      (message `/Game/99_Testarea/Giuseppe/Blueprints/Interfaces/BPI_AnimTraps.StartNightPhase` (`SkeletalMeshComponent.GetAnimInstance` (`/Game/99_Testarea/Giuseppe/Blueprints/Trap/BP_TestTrap.SkeletalMesh_Trap` _array_element)))
      (message `/Game/99_Testarea/Giuseppe/Blueprints/Interfaces/BPI_AnimTraps.StartNightPhase` _array_element))))

(fn `Start Day Phase`
  (bind _daystate (`self.DayState`))
  (`ActorComponent.SetActive` (`self.DaySoundObject`) true false)
  (`ActorComponent.SetActive` (`self.NightSoundObject`) false false)
  (if (`self.FinalWave?`)
    (`/Game/06_UI/WB_HUD.GameOverLAY` (`self.HUD`) "YOU WIN!!!")
    (else
      (`/Game/03_GameplayAssets/03_Artefacts/BP_ArtefactSpawner.SpawnALLArtefacts` (`self.ArtefactManager`) (`/Game/03_GameplayAssets/05_Portals/BP_EnemySpawnManager.WaveCounter` (`self.SpawnManager`)))
      (`/Game/03_GameplayAssets/03_Artefacts/BP_ArtefactSpawner.DeactivateBarriers` (`self.ArtefactManager`))
      (set `self.DayTime` 0.0)
      (set `self.DayState` "NewEnumerator0")
      (`self.SetLight` (`self.DayLight`))
      (`self.SetActorTickEnabled` true)
      (`/Game/06_UI/WB_HUD.StartDayphase` (`self.HUD`))
      (`/MoveIt/Example/BP_MoveIt_ExampleCharacter.AllowBuildingMode` (`self.Player`))
      (`/Game/99_Testarea/Giuseppe/Blueprints/BP_Grid.CallCycleChange` (`self.Grid`) _daystate)
      (`KismetSystemLibrary.PrintString` (`|GetEnumeratorNameAsString` _daystate))
      (bind _outactors (`GameplayStatics.GetAllActorsOfClass` "/Game/99_Testarea/Giuseppe/Blueprints/Trap/BP_TestTrap.BP_TestTrap_C"))
      (for _array_element _outactors
        (message `/Game/99_Testarea/Giuseppe/Blueprints/Interfaces/BPI_AnimTraps.StartDayPhase` (`SkeletalMeshComponent.GetAnimInstance` (`/Game/99_Testarea/Giuseppe/Blueprints/Trap/BP_TestTrap.SkeletalMesh_Trap` _array_element)))
        (message `/Game/99_Testarea/Giuseppe/Blueprints/Interfaces/BPI_AnimTraps.StartDayPhase` _array_element)))))

(fn `StartDayNigthCyle`
  (bind _grid (`self.Grid`))
  (if (`|EnumEquality` (`self.DayState`) "NewEnumerator2")
    (`ActorComponent.SetActive` (`self.DaySoundObject`) true false)
    (bind _returnvalue (`GameplayStatics.GetActorOfClass` "/Game/99_Testarea/Markus/PointSystem/BP_PointSystem.BP_PointSystem_C"))
    (`/Game/99_Testarea/Markus/PointSystem/BP_PointSystem.StartPointSystem` _returnvalue)
    (`self.SetActorTickEnabled` true)
    (set `self.DayState` "NewEnumerator0")
    (`/MoveIt/Example/BP_MoveIt_ExampleCharacter.AllowBuildingMode` (`self.Player`))
    (`/Engine/EditorBlueprintResources/StandardMacros.IsValid` _grid
      (:`Is Valid`
        (`/Game/99_Testarea/Giuseppe/Blueprints/BP_Grid.CallCycleChange` _grid (`self.DayState`))
        (bind _outactors (`GameplayStatics.GetAllActorsOfClass` "/Game/99_Testarea/Giuseppe/Blueprints/Trap/BP_TestTrap.BP_TestTrap_C"))
        (for _array_element _outactors
          (message `/Game/99_Testarea/Giuseppe/Blueprints/Interfaces/BPI_AnimTraps.StartDayPhase` (`SkeletalMeshComponent.GetAnimInstance` (`/Game/99_Testarea/Giuseppe/Blueprints/Trap/BP_TestTrap.SkeletalMesh_Trap` _array_element)))
          (message `/Game/99_Testarea/Giuseppe/Blueprints/Interfaces/BPI_AnimTraps.StartDayPhase` _array_element))))))

(fn `UserConstructionScript`
  (bind _returnvalue (`GameplayStatics.GetActorOfClass` "/Game/03_GameplayAssets/05_Portals/BP_EnemySpawnManager.BP_EnemySpawnManager_C"))
  (bind _output_get (set `self.SpawnManager` _returnvalue))
  (set `/Game/03_GameplayAssets/05_Portals/BP_EnemySpawnManager.DayNightCycle` self _output_get))