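; Test enemy pawn that walks to the Nexus to damage it and dies when it hits the player.
; On BeginPlay it registers with BP_SpawnManager, stays invisible for half the spawn timer, then appears and uses AIMoveTo toward the Nexus.
; Hit events apply Nexus damage after a five-second Delay, which throttles repeat hits.
; Hitting the player reports the kill to the SpawnManager, triggers its enemy count check and destroys the enemy.
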(event `self.ReceiveBeginPlay`
  ;[1 1 1] On BeginPlay, get SpawnManager Nexus & Player and start moving towards Nexus after delay
  (`SceneComponent.SetVisibility` (`self.Mesh`) false false)
  (bind _returnvalue (`GameplayStatics.GetActorOfClass` "/Game/TonyTeststuff/BP_SpawnManager.BP_SpawnManager_C"))
  (bind _output_get (set `self.SpawnManager` _returnvalue))
  (`/Game/TonyTeststuff/BP_SpawnManager.AddSpawned` _output_get)
  (`KismetSystemLibrary.Delay` (* (`/Game/TonyTeststuff/BP_SpawnManager.SpawnTimer` (`self.SpawnManager`)) 0.5))
  (`SceneComponent.SetVisibility` (`self.Mesh`) true false)
  (bind _returnvalue_2 (`GameplayStatics.GetActorOfClass` "/MoveIt/Example/BP_MoveIt_ExampleCharacter.BP_MoveIt_ExampleCharacter_C"))
  (set `self.Player` _returnvalue_2)
  (bind _returnvalue_3 (`GameplayStatics.GetActorOfClass` "/Game/TonyTeststuff/BP_Nexus.BP_Nexus_C"))
  (set `self.Nexus` _returnvalue_3)
  (`|AIMoveTo` self (0.0 0.0 0.0) (`self.Nexus`) 0.05))

(event `self.ReceiveHit`
  (params (MyComp :type "PrimitiveComponent Object Reference") (Other :type "Actor Object Reference") (OtherComp :type "PrimitiveComponent Object Reference") (bSelfMoved :type Boolean) (HitLocation :type "Vector Structure") (HitNormal :type "Vector Structure") (NormalImpulse :type "Vector Structure") (Hit :type "HitResult Structure (by ref)"))
  ;[1 1 1] On Hit, check if Nexus & apply damage every 5 seconds, if Player- get destroyed
  (if (== Other (`self.Nexus`))
    (`KismetSystemLibrary.Delay` 5.0)
    (`/Game/TonyTeststuff/BP_Nexus.ReceiveDamage` (`self.Nexus`))
    (elif (== Other (`self.Player`))
      (`/Game/TonyTeststuff/BP_SpawnManager.AddKilled` (`self.SpawnManager`))
      (`/Game/TonyTeststuff/BP_SpawnManager.CheckCurrentEnemies` (`self.SpawnManager`))
      (`self.K2_DestroyActor`))))

(event `self.CapsuleComponent.OnComponentBeginOverlap`
  (params (OverlappedComponent :type "PrimitiveComponent Object Reference") (OtherActor :type "Actor Object Reference") (OtherComp :type "PrimitiveComponent Object Reference") (OtherBodyIndex :type Integer) (bFromSweep :type Boolean) (SweepResult :type "HitResult Structure (by ref)")))

(fn `UserConstructionScript`)