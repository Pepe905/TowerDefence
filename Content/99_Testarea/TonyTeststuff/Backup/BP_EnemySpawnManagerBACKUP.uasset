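; Manager actor that runs enemy waves from active portals, using an object pool of BP_EnemyTest actors spawned below the map in batches of 50.
; Each wave raises the spawn count and moves pooled enemies to portals; elite rounds spawn one elite per boss-capable portal instead.
; Despawned enemies return to the passive pool.
; When none remain, it starts the day phase and raises max health of pooled enemies.
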(event `self.ReceiveBeginPlay`
  ;[1 1 1] Setup initial PASSIVE EnemyPool
  (`self.IncreaseEnemyPool`))

(event `NextWave`
  (params (`EliteRound?` :type Boolean))
  ;[1 1 1] Call Spawn of next wave on all active portals
  (`/Engine/EditorBlueprintResources/StandardMacros.IncrementInt` (`self.WaveCounter`)
    (:`  `
      (`/Engine/EditorBlueprintResources/StandardMacros.IncrementInt` (`self.EnemyToSpawn`)
        (:`  `
          (for _array_element (`self.PortalActive`)
            (bind _output_get (set `self.PortalSpawning` _array_element))
            (`/Game/03_GameplayAssets/05_Portals/BP_Portal.CheckPaths` _output_get)
            (`self.SpawnEnemiesAtPortal` `EliteRound?`))
          (set `self.EnemyLeft` (+ (`self.EnemyLeft`) (`KismetArrayLibrary.Array_Length` (`self.EnemyPoolACTIVE`)))))))))

(fn `CheckEliteEnemySpawning`
  (if (`/Game/03_GameplayAssets/05_Portals/BP_Portal.CanSpawnBossEnemy?` (`self.PortalSpawning`))
    (`/Engine/EditorBlueprintResources/StandardMacros.IsValid` (`/Game/03_GameplayAssets/05_Portals/BP_Portal.EliteEnemy` (`self.PortalSpawning`))
      (:`Is Valid`
        _)
      (:`Is Not Valid`
        (`self.InitEliteEnemy` (`self.PortalSpawning`)))))
  (return))

(fn `CheckEnemiesLeft`
  (`self.UpdateEnemyLeft`)
  (if (<= (`self.EnemyLeft`) 0)
    (`/Game/99_Testarea/Markus/BP_DayNightCycle.Start Day Phase` (`self.DayNightCycle`))
    (for _array_element (`self.EnemyPoolPASSIVE`)
      (bind _ac_healthmanagement (`/Game/04_Characters/02_Enemies/BP_EnemyTest.AC_Healthmanagement` _array_element))
      (set `/Game/99_Testarea/TonyTeststuff/AC_Healthmanagement.MaxHealth` (+ (`self.EnemyHealthIncreasePerRound`) (`/Game/99_Testarea/TonyTeststuff/AC_Healthmanagement.MaxHealth` _ac_healthmanagement)) _ac_healthmanagement))))

(fn `DespawnEnemies`
  (params (Enemy :type "/Game/04_Characters/02_Enemies/BP_EnemyTest Object Reference"))
  (locals (EnemyTmp :type "/Game/04_Characters/02_Enemies/BP_EnemyTest Object Reference"))
  (set `local.EnemyTmp` Enemy)
  (if (== (`GameplayStatics.GetObjectClass` Enemy) "/Game/04_Characters/02_Enemies/BP_EnemyTest.BP_EnemyTest_C")
    (`KismetArrayLibrary.Array_Remove` (`self.EnemyPoolACTIVE`) (`KismetArrayLibrary.Array_Find` (`self.EnemyPoolACTIVE`) (`local.EnemyTmp`)))
    (`KismetArrayLibrary.Array_Add` (`self.EnemyPoolPASSIVE`) (`local.EnemyTmp`))))

(fn `IncreaseEnemyPool`
  (bind _returnvalue (`self.GetTransform` self))
  (for _ (range 50)
    (bind _returnvalue_2 (`|SpawnActorFromClass` "/Game/04_Characters/02_Enemies/BP_EnemyTest.BP_EnemyTest_C" (`KismetMathLibrary.MakeTransform` (`KismetMathLibrary.MakeVector` (.x (.location _returnvalue)) (.y (.location _returnvalue)) -1000.0) (.rotation _returnvalue) (.scale _returnvalue)) "AdjustIfPossibleButAlwaysSpawn" "OverrideRootScale" null null))
    (`/Game/04_Characters/02_Enemies/BP_EnemyTest.SetupEnemy` _returnvalue_2)
    (`KismetArrayLibrary.Array_Add` (`self.EnemyPoolPASSIVE`) _returnvalue_2)))

(fn `InitEliteEnemy`
  (params (PortalConnectedToEliteEnemy :type "/Game/03_GameplayAssets/05_Portals/BP_Portal Object Reference"))
  (bind _returnvalue (`self.GetTransform` PortalConnectedToEliteEnemy))
  (bind _returnvalue_2 (`|SpawnActorFromClass` "/Game/04_Characters/02_Enemies/BP_EliteEnemyTest.BP_EliteEnemyTest_C" (`KismetMathLibrary.MakeTransform` (`KismetMathLibrary.MakeVector` (.x (.location _returnvalue)) (.y (.location _returnvalue)) -1000.0) (.rotation _returnvalue) (.scale _returnvalue)) "AdjustIfPossibleButAlwaysSpawn" "OverrideRootScale" null null))
  (`/Game/04_Characters/02_Enemies/BP_EnemyTest.SetupEnemy` _returnvalue_2)
  (set `/Game/03_GameplayAssets/05_Portals/BP_Portal.EliteEnemy` _returnvalue_2 PortalConnectedToEliteEnemy))

(fn `SpawnEnemiesAtPortal`
  (params (`EliteRound?` :type Boolean))
  (locals (EnemyTmp :type "/Game/04_Characters/02_Enemies/BP_EnemyTest Object Reference") (EnemyToSpawnHere :type "Array of /Game/04_Characters/02_Enemies/BP_EnemyTest Object Reference"))
  (bind _output (`|GetArrayItem` (`self.EnemyPoolPASSIVE`)))
  (if `EliteRound?`
    (`self.CheckEliteEnemySpawning`)
    (`/Game/03_GameplayAssets/05_Portals/BP_Portal.SpawnEnemies` (`self.PortalSpawning`) true)
    (else
      (for _ (range (+ (+ (`self.EnemyToSpawn`) (`/Game/03_GameplayAssets/05_Portals/BP_Portal.SpawnCountModifier` (`self.PortalSpawning`))) 1))
        (if (`KismetSystemLibrary.IsValid` _output)
          (set `local.EnemyTmp` _output)
          (`KismetArrayLibrary.Array_Remove` (`self.EnemyPoolPASSIVE`))
          (`KismetArrayLibrary.Array_Add` (`self.EnemyPoolACTIVE`) (`local.EnemyTmp`))
          (`KismetArrayLibrary.Array_Add` (`/Game/03_GameplayAssets/05_Portals/BP_Portal.EnemiesToSpawn` (`self.PortalSpawning`)) (`local.EnemyTmp`))
          (else
            (`self.IncreaseEnemyPool`))))
      (`/Game/03_GameplayAssets/05_Portals/BP_Portal.SpawnEnemies` (`self.PortalSpawning`) false))))

(fn `UpdateEnemyLeft`
  (`/Engine/EditorBlueprintResources/StandardMacros.DecrementInt` (`self.EnemyLeft`)
    (:`  `
      (`/Engine/EditorBlueprintResources/StandardMacros.IncrementInt` (`self.GlobalEnemyCounter`)))))

(fn `UserConstructionScript`)