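; BP_Artefact is a collectible artefact that plays an attenuated sound at its location from BeginPlay.
; When the example player character hits its cube, it plays collect and Nox-appearance sounds, reports itself to the artefact spawner, stops its main sound and destroys itself.
; Two functions, not called within this Blueprint, toggle the night-lock barrier's visibility and collision between blocking and ignored.
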(event `self.ReceiveBeginPlay`
  ;[1 1 1] BeginPlay & Play Sound
  (bind _returnvalue (`GameplayStatics.GetActorOfClass` "/MoveIt/Example/BP_MoveIt_ExampleCharacter.BP_MoveIt_ExampleCharacter_C"))
  (set `self.Player` _returnvalue)
  (bind _returnvalue_2 (`GameplayStatics.GetActorOfClass` "/Game/03_GameplayAssets/03_Artefacts/BP_ArtefactSpawner.BP_ArtefactSpawner_C"))
  (set `self.ArtefactSpawner` _returnvalue_2)
  (bind _returnvalue_3 (`GameplayStatics.SpawnSoundAtLocation` "/Game/07_Audio/Artefakt/ArtefactMainSound.ArtefactMainSound" (`SceneComponent.K2_GetComponentLocation` (`self.Cube`)) (struct) 2.5 1.0 0.0 "/Game/07_Audio/MyAttenuation.MyAttenuation" null)))

(event `self.ReceiveHit`
  (params (MyComp :type "PrimitiveComponent Object Reference") (Other :type "Actor Object Reference") (OtherComp :type "PrimitiveComponent Object Reference") (bSelfMoved :type Boolean) (HitLocation :type "Vector Structure") (HitNormal :type "Vector Structure") (NormalImpulse :type "Vector Structure") (Hit :type "HitResult Structure (by ref)"))
  ;[1 1 1] OnHitEvent
  (if (and (== MyComp (`self.Cube`)) (== Other (`self.Player`)))
    (`GameplayStatics.SpawnSoundAtLocation` "/Game/07_Audio/Artefakt/ArtefactCollect.ArtefactCollect" (`SceneComponent.K2_GetComponentLocation` (`self.Cube`)) (struct) 0.2 1.0 0.0 "/Game/07_Audio/MyAttenuation.MyAttenuation" null)
    (`GameplayStatics.SpawnSound2D` "/Game/07_Audio/Enemies/Nox-Appears.Nox-Appears" 1.3 1.0 0.0 null)
    (`/Game/03_GameplayAssets/03_Artefacts/BP_ArtefactSpawner.GetCollectedArtefacts` (`self.ArtefactSpawner`) self)
    (`AudioComponent.Stop` (stale `self.ReceiveBeginPlay` _returnvalue_3))
    (`self.K2_DestroyActor`)))

(fn `ActivateBarriere`
  (`SceneComponent.SetVisibility` (`self.BarrierLockNight`) true false)
  (`PrimitiveComponent.SetCollisionResponseToAllChannels` (`self.BarrierLockNight`) "ECR_Block"))

(fn `DeactivateBarriere`
  (`SceneComponent.SetVisibility` (`self.BarrierLockNight`) false false)
  (`PrimitiveComponent.SetCollisionResponseToAllChannels` (`self.BarrierLockNight`) "ECR_Ignore"))

(fn `UserConstructionScript`)