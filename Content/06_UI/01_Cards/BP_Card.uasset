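; BP_Card is a collectible card actor that notifies BP_MoveIt_ExampleCharacter when that character overlaps it.
; SpawnCard loads details and rarity color from DT_Cards by ID, then shows the widget with query collision; InitCard links WB_Cards back to the actor.
; Collecting hides the widget and disables its collision, while discarding also reports to CardManager.
; CardUsed is empty, and the drop-chance rarity coloring is disconnected.
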(event `self.ReceiveActorBeginOverlap`
  (params (OtherActor :type "Actor Object Reference"))
  (if (== (`GameplayStatics.GetObjectClass` OtherActor) "/MoveIt/Example/BP_MoveIt_ExampleCharacter.BP_MoveIt_ExampleCharacter_C")
    (message `/Game/06_UI/01_Cards/BPI_CardUsage.CollectedCard` OtherActor self)))

(event `/Game/06_UI/01_Cards/BPI_CardUsage.CollectedCard`
  (params (CardCollected :type "/Game/06_UI/01_Cards/BP_Card Object Reference"))
  (`self.CardCollected`)
  (`KismetSystemLibrary.PrintString` "PLAYER COLLECTS CARD"))

(event `/Game/06_UI/01_Cards/BPI_CardUsage.DiscardCard`
  (`self.DespawnCard`))

(fn `CardCollected`
  (`PrimitiveComponent.SetCollisionEnabled` (`self.Widget`) "NoCollision")
  (`SceneComponent.SetVisibility` (`self.Widget`) false false))

(fn `CardUsed`)

(fn `DespawnCard`
  (`PrimitiveComponent.SetCollisionEnabled` (`self.Widget`) "NoCollision")
  (`SceneComponent.SetVisibility` (`self.Widget`) false false)
  (`/Game/06_UI/01_Cards/BP_CardManager.DespawnCard` (`self.CardManager`) self))

(fn `InitCard`
  (locals (Rarity :type Integer) (DropChance :type "Float (double-precision)"))
  (bind _aswb_cards (cast `/Game/06_UI/01_Cards/WB_Cards` (`WidgetComponent.GetWidget` (`self.Widget`))))
  (set `/Game/06_UI/01_Cards/WB_Cards.OwningCard` self _aswb_cards))

(fn `SpawnCard`
  (params (CardID :type Name))
  (bind _returnvalue (`|GetDataTableRow` "/Game/06_UI/01_Cards/DT_Cards.DT_Cards" CardID)
    (:`then`
      (bind _output_get (set `self.CardDetails` _returnvalue))
      (set `self.RarityColorDisplay` (`.CardColor_53_2116D8C444AC916E4AD1D9AC556F8C6A` (break `/Game/06_UI/01_Cards/ST_Cards` _output_get)))
      (`PrimitiveComponent.SetCollisionEnabled` (`self.Widget`) "QueryOnly")
      (`SceneComponent.SetVisibility` (`self.Widget`) true false))))

(fn `UserConstructionScript`)