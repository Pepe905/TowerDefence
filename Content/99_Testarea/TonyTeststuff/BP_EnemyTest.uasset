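; BP_EnemyTest is an enemy character that walks to BP_Nexus, damaging it and self-destructing on contact, or damaging the player when it hits them.
; It registers with BP_SpawnManager and stays hidden for half the spawn timer before AIMoveTo starts.
; A timed slowdown scales and restores walk speed, while damage reveals and updates a health bar widget.
; Death updates spawn counts and gives Nexus mana, awarding points unless self-destructed.
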(event `self.ReceiveBeginPlay`
  ;[1 1 1] On BeginPlay, get SpawnManager Nexus & Player and start moving towards Nexus after delay
  (set `self.SaveMaxWalkSpeed` (`CharacterMovementComponent.MaxWalkSpeed` (`self.MICharacterMovement`)))
  (`SceneComponent.SetVisibility` (`self.Mesh`) false false)
  (`SceneComponent.SetVisibility` (`self.Aura`) false false)
  (bind _returnvalue (`GameplayStatics.GetActorOfClass` "/Game/99_Testarea/TonyTeststuff/BP_SpawnManager.BP_SpawnManager_C"))
  (bind _output_get (set `self.SpawnManager` _returnvalue))
  (`/Game/99_Testarea/TonyTeststuff/BP_SpawnManager.AddSpawned` _output_get)
  (`KismetSystemLibrary.Delay` (* (`/Game/99_Testarea/TonyTeststuff/BP_SpawnManager.SpawnTimer` (`self.SpawnManager`)) 0.5))
  (`SceneComponent.SetVisibility` (`self.Mesh`) true false)
  (`SceneComponent.SetVisibility` (`self.Aura`) true false)
  (bind _returnvalue_2 (`GameplayStatics.GetActorOfClass` "/MoveIt/Example/BP_MoveIt_ExampleCharacter.BP_MoveIt_ExampleCharacter_C"))
  (set `self.Player` _returnvalue_2)
  (bind _returnvalue_3 (`GameplayStatics.GetActorOfClass` "/Game/99_Testarea/TonyTeststuff/BP_Nexus.BP_Nexus_C"))
  (set `self.Nexus` _returnvalue_3)
  (`|AIMoveTo` null (0.0 0.0 0.0) (`self.Nexus`) 0.5
    (:`then`
      (`self.UpdateHealthbar`))))

(event `self.SlowDown`
  (params (Slowdown :type "Float (double-precision)") (SlowdonDuration :type "Float (double-precision)"))
  ;[1 1 1] Slowdown of Speed & Restore Speed
  (`KismetSystemLibrary.K2_SetTimerDelegate` (delegate `RestoreSpeed`) SlowdonDuration)
  (set `CharacterMovementComponent.MaxWalkSpeed` (* Slowdown (`self.SaveMaxWalkSpeed`)) (`self.MICharacterMovement`)))

(event `RestoreSpeed`
  ;[1 1 1] Slowdown of Speed & Restore Speed
  (set `CharacterMovementComponent.MaxWalkSpeed` (`self.SaveMaxWalkSpeed`) (`self.MICharacterMovement`)))

(event `self.ReceiveHit`
  (params (MyComp :type "PrimitiveComponent Object Reference") (Other :type "Actor Object Reference") (OtherComp :type "PrimitiveComponent Object Reference") (bSelfMoved :type Boolean) (HitLocation :type "Vector Structure") (HitNormal :type "Vector Structure") (NormalImpulse :type "Vector Structure") (Hit :type "HitResult Structure (by ref)"))
  (bind _player (`self.Player`))
  (bind _nexus (`self.Nexus`))
  ;[1 1 1] On Hit, check if Player / Nexus & apply damage/ destory
  (if (== Other _nexus)
    (`/Game/99_Testarea/TonyTeststuff/AC_Healthmanagement.TakeDamage` (`/Game/99_Testarea/TonyTeststuff/BP_Nexus.AC_Healthmanagement` _nexus) 25.0)
    (`self.Death` true)
    (elif (== Other _player)
      (`/Game/99_Testarea/TonyTeststuff/AC_Healthmanagement.TakeDamage` (`/MoveIt/Example/BP_MoveIt_ExampleCharacter.AC_Healthmanagement` _player) 25.0))))

(event `self.Death`
  (params (selfDescruct :type Boolean))
  ;[1 1 1] Selfdestruction (either because Enemy arrived at Nexus or was defeated)
  (if (not selfDescruct)
    (bind _returnvalue (`GameplayStatics.GetActorOfClass` "/Game/99_Testarea/Markus/PointSystem/BP_PointSystem.BP_PointSystem_C"))
    (`/Game/99_Testarea/Markus/PointSystem/BP_PointSystem.EnemyDeath` _returnvalue (`self.Points`)))
  (`/Game/99_Testarea/TonyTeststuff/BP_SpawnManager.AddKilled` (`self.SpawnManager`))
  (`/Game/99_Testarea/TonyTeststuff/BP_SpawnManager.CheckCurrentEnemies` (`self.SpawnManager`))
  (`/Game/99_Testarea/TonyTeststuff/BP_Nexus.ManaGain` (`self.Nexus`) 5.0)
  (`self.K2_DestroyActor`))

(event `self.DmgTaken`
  ;[1 1 1] Update Healthbar
  (`SceneComponent.SetVisibility` (`self.Healthbar`) true false)
  (`self.UpdateHealthbar`))

(fn `UpdateHealthbar`
  (bind _aswb_enemy_healthbar (cast `/Game/99_Testarea/TonyTeststuff/WB_EnemyHealthbar` (`WidgetComponent.GetUserWidgetObject` (`self.Healthbar`)))
    (:`then`
      (set `/Game/99_Testarea/TonyTeststuff/WB_EnemyHealthbar.CurrentHealth` (/ (`/Game/99_Testarea/TonyTeststuff/AC_Healthmanagement.CurrentHealth` (`self.AC_Healthmanagement`)) (`/Game/99_Testarea/TonyTeststuff/AC_Healthmanagement.MaxHealth` (`self.AC_Healthmanagement`))) _aswb_enemy_healthbar))
    (:`CastFailed`
      (`KismetSystemLibrary.PrintString` "NO ENEMY HEALTHBAR"))))

(fn `UserConstructionScript`)