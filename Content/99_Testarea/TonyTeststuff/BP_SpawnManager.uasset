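; Wave spawn manager, in a test area, that spawns test enemies at active portals and works with the day/night cycle.
; Setup starts the cycle before the first wave, and each wave loops through portals, offsetting spawn counts by loop order and each portal's modifier.
; External events update spawned and killed counters.
; When these match on a check, the day phase starts and the base enemy count grows.
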(event `SpawnSetup`
  ;[1 1 1] Prepare new Wave, adjust counter & loop through all active Portals to spawn new wave
  (if (not (> (`self.WaveCounter`) 0))
    (`/Game/99_Testarea/Markus/BP_DayNightCycle.StartDayNigthCyle` (`self.DayNightCycle`))))

(event `NextWave`
  ;[1 1 1] Comment
  (`/Engine/EditorBlueprintResources/StandardMacros.IncrementInt` (`self.WaveCounter`)
    (:`  `
      (`KismetSystemLibrary.PrintString` (`KismetStringLibrary.Conv_IntToString` (`self.WaveCounter`)))
      (`KismetSystemLibrary.PrintString` "WAVE")
      (for _array_element (`self.PortalActive`)
        (set `self.PortalSpawning` _array_element)
        (`/Engine/EditorBlueprintResources/StandardMacros.IncrementInt` (`self.SpawnModifierIntern`)
          (:`  `
            (`self.SpawnEnemies`))))
      (set `self.SpawnModifierIntern` 0)
      (`KismetSystemLibrary.PrintString` (`KismetStringLibrary.Conv_IntToString` (`self.EnemySpawned`)))
      (`KismetSystemLibrary.PrintString` "ENEMIES SPAWNED"))))

(event `SpawnEnemies`
  ;[1 1 1] Spawn Enemies with adjusted Amount at current Portal & set delays for Enemies
  (for _ (range (+ (+ (- (`self.EnemyToSpawn`) (`self.SpawnModifierIntern`)) (`/Game/99_Testarea/TonyTeststuff/BP_Portal.SpawnCountModifier` (`self.PortalSpawning`))) 1))
    (`/Engine/EditorBlueprintResources/StandardMacros.IncrementFloat` (`self.SpawnTimer`)
      (:`  `
        (`|SpawnActorFromClass` "/Game/99_Testarea/TonyTeststuff/BP_EnemyTest.BP_EnemyTest_C" (`self.GetTransform` (`self.PortalSpawning`)) "Undefined" "OverrideRootScale" null null))))
  (set `self.SpawnTimer` 0.0)
  (set `self.EnemiesKilled` 0))

(event `CheckCurrentEnemies`
  ;[1 1 1] Check if all current enemies have been spawned
  (if (== (`self.EnemySpawned`) (`self.EnemiesKilled`))
    (`/Game/99_Testarea/Markus/BP_DayNightCycle.StartDayPhase` (`self.DayNightCycle`))
    (set `self.EnemySpawned` 0)
    (`/Engine/EditorBlueprintResources/StandardMacros.IncrementInt` (`self.EnemyToSpawn`))))

(event `AddSpawned`
  ;[1 1 1] Increment Spawned & Killed Enemies
  (`/Engine/EditorBlueprintResources/StandardMacros.IncrementInt` (`self.EnemySpawned`)
    (:`  `
      (`self.UpdateEnemyLeft`))))

(event `AddKilled`
  ;[1 1 1] Increment Spawned & Killed Enemies
  (`/Engine/EditorBlueprintResources/StandardMacros.IncrementInt` (`self.EnemiesKilled`)
    (:`  `
      (`self.UpdateEnemyLeft`))))

(fn `UpdateEnemyLeft`
  (set `self.EnemyLeft` (- (`self.EnemySpawned`) (`self.EnemiesKilled`))))

(fn `UserConstructionScript`)