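; BP_Door is a test door actor that opens when the player hits it during one specific day state.
; On BeginPlay it caches the player character and the BP_DayNightCycle actor.
; On Hit by the player in that state, it hides its cube, calls Activation on every linked portal, prints a debug message and destroys itself.
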(event `self.ReceiveBeginPlay`
  ;[1 1 1] On BeginPlay, get Player & DayNightCycle
  (bind _returnvalue (`GameplayStatics.GetActorOfClass` "/MoveIt/Example/BP_MoveIt_ExampleCharacter.BP_MoveIt_ExampleCharacter_C"))
  (set `self.Player` _returnvalue)
  (bind _returnvalue_2 (`GameplayStatics.GetActorOfClass` "/Game/99_Testarea/Markus/BP_DayNightCycle.BP_DayNightCycle_C"))
  (set `self.DayNightCycle` _returnvalue_2))

(event `self.ReceiveHit`
  (params (MyComp :type "PrimitiveComponent Object Reference") (Other :type "Actor Object Reference") (OtherComp :type "PrimitiveComponent Object Reference") (bSelfMoved :type Boolean) (HitLocation :type "Vector Structure") (HitNormal :type "Vector Structure") (NormalImpulse :type "Vector Structure") (Hit :type "HitResult Structure (by ref)"))
  ;[1 1 1] On Open, Activate all connected Portals & Destroy self afterwards
  (if (== Other (`self.Player`))
    (if (`|EnumEquality` (`/Game/99_Testarea/Markus/BP_DayNightCycle.DayState` (`self.DayNightCycle`)) "NewEnumerator0")
      (`SceneComponent.SetVisibility` (`self.Cube`) false false)
      (for _array_element (`self.Portal`)
        (`/Game/99_Testarea/TonyTeststuff/BP_Portal.Activation` _array_element))
      (`KismetSystemLibrary.PrintString` "DOOR OPEN")
      (`self.K2_DestroyActor`))))

(fn `UserConstructionScript`)