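; Component that scatters artefacts across the level at random when play begins.
; On BeginPlay it gathers every BP_ArtefactLocation actor, then spawns ArtefactCount BP_Artefact actors, each raised above a randomly picked location.
; Each used location is removed from the pool so none repeats, with no check that enough locations exist.
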(event `self.ReceiveBeginPlay`
  (bind (_returnvalue_x _returnvalue_y _returnvalue_z) (`KismetMathLibrary.BreakVector` (`Actor.K2_GetActorLocation` (`|GetArrayItem` (`self.Spawn Locations`) (`self.RdmTmpIndex`)))))
  (bind _outactors (`GameplayStatics.GetAllActorsOfClass` "/Game/03_GameplayAssets/03_Artefacts/BP_ArtefactLocation.BP_ArtefactLocation_C"))
  (set `self.Spawn Locations` _outactors)
  (for _ (range 1 (+ (`self.ArtefactCount`) 1))
    (set `self.RdmTmpIndex` (`KismetMathLibrary.RandomInteger` (`KismetArrayLibrary.Array_Length` (`self.Spawn Locations`))))
    (`|SpawnActorFromClass` "/Game/03_GameplayAssets/03_Artefacts/BP_Artefact.BP_Artefact_C" (`KismetMathLibrary.Conv_VectorToTransform` (`KismetMathLibrary.MakeVector` _returnvalue_x _returnvalue_y (+ _returnvalue_z 500.0))) "AdjustIfPossibleButAlwaysSpawn" "OverrideRootScale" null null)
    (`KismetArrayLibrary.Array_Remove` (`self.Spawn Locations`) (`self.RdmTmpIndex`))))