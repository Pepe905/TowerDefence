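; Artefact spawner that places collectible artefacts by round and tracks progress toward winning.
; At four milestone rounds it spawns one artefact above a random location from the matching tier, mapping it to that location's connected portal.
; Collecting one enables boss spawning at its portal, then either shows the win screen when all are collected or conditionally skips the day phase.
; It also toggles barriers on all active artefacts.
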(event `self.ReceiveBeginPlay`
  (bind _returnvalue (`GameplayStatics.GetActorOfClass` "/MoveIt/Example/BP_MoveIt_ExampleCharacter.BP_MoveIt_ExampleCharacter_C"))
  (set `self.Player` _returnvalue))

(fn `ActivateBarriers`
  (for _array_element (`self.ActiveArtefacts`)
    (`/Game/03_GameplayAssets/03_Artefacts/BP_Artefact.ActivateBarriere` _array_element)))

(fn `DeactivateBarriers`
  (for _array_element (`self.ActiveArtefacts`)
    (`/Game/03_GameplayAssets/03_Artefacts/BP_Artefact.DeactivateBarriere` _array_element)))

(fn `GetCollectedArtefacts`
  (params (CollectedArtefact :type "/Game/03_GameplayAssets/03_Artefacts/BP_Artefact Object Reference"))
  (`/Game/03_GameplayAssets/05_Portals/BP_Portal.EnableBossEnemySpawn` (`BlueprintMapLibrary.Map_Find` (`self.MAPArtefactPortal`) CollectedArtefact))
  (`KismetArrayLibrary.Array_RemoveItem` (`self.ActiveArtefacts`) CollectedArtefact)
  (`/Engine/EditorBlueprintResources/StandardMacros.IncrementInt` (`self.ArtefactCollected`)
    (:`  `
      (if (<= (`self.ArtefactCount`) (`self.ArtefactCollected`))
        (`/Game/06_UI/WB_HUD.GameOverLAY` (`/MoveIt/Example/BP_MoveIt_ExampleCharacter.DemoWidget` (`self.Player`)) "YOU COLLECTED ALL ARTEFACTS!  \nYOU WIN!")
        (elif (`|EnumEquality` (`/Game/99_Testarea/Markus/BP_DayNightCycle.DayState` (`/MoveIt/Example/BP_MoveIt_ExampleCharacter.DayNightCycle` (`self.Player`))) "NewEnumerator0")
          (`/Game/99_Testarea/Markus/BP_DayNightCycle.SkipDayPhase` (`/MoveIt/Example/BP_MoveIt_ExampleCharacter.DayNightCycle` (`self.Player`)) true)
          (`KismetSystemLibrary.PrintString` "DAYSKIP ARTEFACTCOLLECT" true true (struct :`R` 1.0 :`G` 0.069327 :`A` 1.0)))))))

(fn `SpawnALLArtefacts`
  (params (Round :type Integer))
  (switch `int` Round
    (:`1`
      (`self.SpawnONEArtefactInTier` (`self.ArtefactLocations_Tier1`)))
    (:`4`
      (`self.SpawnONEArtefactInTier` (`self.ArtefactLocations_Tier2`)))
    (:`7`
      (`self.SpawnONEArtefactInTier` (`self.ArtefactLocations_Tier3`)))
    (:`10`
      (`self.SpawnONEArtefactInTier` (`self.ArtefactLocations_Tier4`))))
  (`KismetSystemLibrary.PrintString` "ARTEFACT SPAWNED" true true (struct :`R` 1.0 :`B` 0.833344 :`A` 1.0)))

(fn `SpawnONEArtefactInTier`
  (params (TierToSpawn :type "Array of /Game/03_GameplayAssets/03_Artefacts/BP_ArtefactLocation Object Reference"))
  (bind (_returnvalue_x _returnvalue_y _returnvalue_z) (`KismetMathLibrary.BreakVector` (`self.K2_GetActorLocation` (`self.TmpArtefactLocation`))))
  (set `self.TmpArtefactLocation` (`KismetArrayLibrary.Array_Random` TierToSpawn))
  (set `/Game/03_GameplayAssets/03_Artefacts/BP_ArtefactLocation.HasArtefact` true (`self.TmpArtefactLocation`))
  (bind _returnvalue (`|SpawnActorFromClass` "/Game/03_GameplayAssets/03_Artefacts/BP_Artefact.BP_Artefact_C" (`KismetMathLibrary.MakeTransform` (`KismetMathLibrary.MakeVector` _returnvalue_x _returnvalue_y (+ _returnvalue_z (`self.HeightOffsetToSpawnLocation`)))) "AdjustIfPossibleButAlwaysSpawn" "OverrideRootScale" null null))
  (`BlueprintMapLibrary.Map_Add` (`self.MAPArtefactPortal`) _returnvalue (`/Game/03_GameplayAssets/03_Artefacts/BP_ArtefactLocation.ConnectedPortal` (`self.TmpArtefactLocation`)))
  (`KismetArrayLibrary.Array_Add` (`self.ActiveArtefacts`) _returnvalue))

(fn `UserConstructionScript`)