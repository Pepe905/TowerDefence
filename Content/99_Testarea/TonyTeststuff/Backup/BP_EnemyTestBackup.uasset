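; Pooled enemy (backup test Blueprint) that follows spline paths toward the Nexus, damaging the player within its aura.
; Tick advances distance along path parts, supporting reverse travel and temporary dodge splines that rejoin the main path.
; Reaching the Nexus damages it and self-destructs; other deaths also drop cards and award points.
; Despawning grants Nexus mana, notifies the spawn manager, and parks the actor underground with tick and collision off until Activate.
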(event `Activate`
  ;[1 1 1] Activate Enemy on Spawning
  (`self.ResetHealthbar`)
  (`self.SetCollision` true)
  (`self.SetActorTickEnabled` true)
  (`ActorComponent.SetComponentTickEnabled` (`self.AC_Healthmanagement`) true)
  (`self.UpdateHealthbar`))

(event `/Game/99_Testarea/TonyTeststuff/BPI_ActorStateChange.SlowDown`
  (params (Slowdown :type "Float (double-precision)") (SlowdonDuration :type "Float (double-precision)"))
  ;[1 1 1] Slowdown of Speed & Restore Speed
  (`KismetSystemLibrary.K2_SetTimerDelegate` (delegate `RestoreSpeed`) SlowdonDuration)
  (set `self.MoveSpeed` (* Slowdown (`self.SaveMaxWalkSpeed`))))

(event `RestoreSpeed`
  ;[1 1 1] Slowdown of Speed & Restore Speed
  (set `self.MoveSpeed` (`self.SaveMaxWalkSpeed`)))

(event `/Game/99_Testarea/TonyTeststuff/BPI_ActorStateChange.DmgTaken`
  ;[1 1 1] On Damage Taken, Update Healthbar
  (`SceneComponent.SetVisibility` (`self.Healthbar`) true false)
  (`self.UpdateHealthbar`))

(event `/Game/99_Testarea/TonyTeststuff/BPI_ActorStateChange.Death`
  (params (selfDescruct :type Boolean))
  ;[1 1 1] Selfdestruction (either because Enemy arrived at Nexus or was defeated)
  (`self.DYINGFunction` selfDescruct))

(event `self.ReceiveTick`
  (params (DeltaSeconds :type "Float (single-precision)"))
  ;[1 1 1] EventTick - Movement & DistanceCheck
  (`self.MoveAlongSpline` DeltaSeconds)
  (`self.UpdateDistances` DeltaSeconds))

(fn `CalculateDistanceAlongSpline`
  (params (deltaTime :type "Float (double-precision)"))
  (set `self.DistanceAlongSpline` (+ (* (`self.MoveSpeed`) deltaTime) (`self.DistanceAlongSpline`))))

(fn `CalculateNewDistanceAlongPath`
  (bind (_pathparts _index) (break `/Game/99_Testarea/Markus/EnemyPathing/ST_Path` (`self.Path`)))
  (bind (_outdistancealongspline _outmaxsplinedistance _change) (`/Game/99_Testarea/Markus/EnemyPathing/BP_PathFunctions.Check Spline Distance` (`self.Path`) (`self.DistanceAlongSpline`) (`self.MaxSplineDistance`)))
  (set `self.DistanceAlongSpline` _outdistancealongspline)
  (set `self.MaxSplineDistance` _outmaxsplinedistance)
  (if _change
    (`self.Check Reverse Travel` (`/Game/99_Testarea/Markus/EnemyPathing/BP_PathParts.Spline` (`|GetArrayItem` _pathparts _index)))))

(fn `Check Reverse Travel`
  (params (spline :type "SplineComponent Object Reference"))
  (bind _returnvalue (`SceneComponent.K2_GetComponentLocation` (`self.CapsuleComponent`)))
  (set `self.ReverseTravel` (< (`KismetMathLibrary.Vector_DistanceSquared` (`SplineComponent.GetLocationAtSplinePoint` spline (- (`SplineComponent.GetNumberOfSplinePoints` spline) 1) "World") _returnvalue) (`KismetMathLibrary.Vector_DistanceSquared` (`SplineComponent.GetLocationAtSplinePoint` spline 0 "World") _returnvalue))))

(fn `DespawnEnemy`
  (bind (_returnvalue_x _returnvalue_y) (`KismetMathLibrary.BreakVector` (`self.K2_GetActorLocation`)))
  (if (not (== (`GameplayStatics.GetObjectClass` self) "/Game/04_Characters/02_Enemies/BP_EliteEnemyTest.BP_EliteEnemyTest_C"))
    (`/Game/03_GameplayAssets/05_Portals/BP_EnemySpawnManager.DespawnEnemies` (`self.SpawnManager`) self))
  (`self.SetCollision` false)
  (`/Game/03_GameplayAssets/05_Portals/BP_EnemySpawnManager.CheckEnemiesLeft` (`self.SpawnManager`))
  (`/Game/03_GameplayAssets/02_Nexus/BP_Nexus.ManaGain` (`self.Nexus`) (`self.Mana Increase`))
  (`self.K2_SetActorLocation` (`KismetMathLibrary.MakeVector` _returnvalue_x _returnvalue_y -1000.0) false true)
  (`self.ResetHealthbar`)
  (`self.SetActorTickEnabled` false)
  (`ActorComponent.SetComponentTickEnabled` (`self.AC_Healthmanagement`) false)
  (set `self.MoveSpeed` (`self.SaveMaxWalkSpeed`)))

(fn `DropCard`
  (`/Game/06_UI/01_Cards/BP_CardManager.CardDropCalculation` (`self.CardManager`) (`SceneComponent.K2_GetComponentLocation` (`self.CapsuleComponent`))))

(fn `DYINGFunction`
  (params (`SelfDestruct?` :type Boolean))
  (if (not `SelfDestruct?`)
    (`self.DropCard`)
    (bind _returnvalue (`GameplayStatics.GetActorOfClass` "/Game/99_Testarea/Markus/PointSystem/BP_PointSystem.BP_PointSystem_C"))
    (`/Game/99_Testarea/Markus/PointSystem/BP_PointSystem.EnemyDeath` _returnvalue (`self.Points`)))
  (`self.DespawnEnemy`))

(fn `GetSpline`
  (returns (spline :type "SplineComponent Object Reference"))
  (locals (outputSpline :type "SplineComponent Object Reference"))
  (bind (_pathparts _index) (break `/Game/99_Testarea/Markus/EnemyPathing/ST_Path` (`self.Path`)))
  (`/Engine/EditorBlueprintResources/StandardMacros.IsValid` (`self.DogeSpline`)
    (:`Is Valid`
      (set `local.outputSpline` (`self.DogeSpline`)))
    (:`Is Not Valid`
      (set `local.outputSpline` (`/Game/99_Testarea/Markus/EnemyPathing/BP_PathParts.Spline` (`|GetArrayItem` _pathparts _index)))))
  (return (`local.outputSpline`)))

(fn `LeaveDogePath`
  (bind (_pathparts _index) (break `/Game/99_Testarea/Markus/EnemyPathing/ST_Path` (`self.Path`)))
  (bind _spline (`/Game/99_Testarea/Markus/EnemyPathing/BP_PathParts.Spline` (`|GetArrayItem` _pathparts _index)))
  (set `self.DistanceAlongSpline` (+ (- (`self.DistanceAlongSpline`) (`self.MaxSplineDistance`)) (`SplineComponent.GetDistanceAlongSplineAtSplineInputKey` _spline (`SplineComponent.FindInputKeyClosestToWorldLocation` _spline (`SplineComponent.GetLocationAtDistanceAlongSpline` (`self.DogeSpline`) (`self.MaxSplineDistance`) "World")))))
  (set `self.MaxSplineDistance` (`SplineComponent.GetSplineLength` _spline))
  (set `self.DogeSpline` null)
  (set `self.ReverseTravel` (`self.ReverseTravelSave`)))

(fn `MoveAlongSpline`
  (params (deltaTime :type "Float (double-precision)"))
  (if (`.IsFree_8_E28C161941444E240D38F3B26AC8EF44` (break `/Game/99_Testarea/Markus/EnemyPathing/ST_Path` (`self.Path`)))
    (`self.CalculateDistanceAlongSpline` deltaTime)
    (`/Engine/EditorBlueprintResources/StandardMacros.IsValid` (`self.DogeSpline`)
      (:`Is Valid`
        (if (>= (`self.DistanceAlongSpline`) (`self.MaxSplineDistance`))
          (`self.LeaveDogePath`)
          (`self.CalculateNewDistanceAlongPath` :!label _label)))
      (:`Is Not Valid`
        (goto _label)))
    (bind _spline (`self.GetSpline`))
    (`self.MoveTransfromBaseOnSplineDistance` _spline)))

(fn `MoveTransfromBaseOnSplineDistance`
  (params (spline :type "SplineComponent Object Reference"))
  (locals (distance :type "Float (double-precision)"))
  (bind _distance (`local.distance`))
  (bind _returnvalue (`SplineComponent.GetTransformAtDistanceAlongSpline` spline _distance "World" false))
  (if (`self.ReverseTravel`)
    (set `local.distance` (- (`self.MaxSplineDistance`) (`self.DistanceAlongSpline`)))
    (set `self.Rotation` (`KismetMathLibrary.Conv_VectorToRotator` (* (`SplineComponent.GetDirectionAtDistanceAlongSpline` spline _distance "World") (-1.0 -1.0 -1.0))))
    (else
      (set `local.distance` (`self.DistanceAlongSpline`))
      (set `self.Rotation` (.rotation _returnvalue))))
  (`self.K2_SetActorTransform` (`KismetMathLibrary.MakeTransform` (`KismetMathLibrary.MakeVector` (.x (.location _returnvalue)) (.y (.location _returnvalue)) (+ (.z (.location _returnvalue)) (`self.SplineZOffset`))) (`self.Rotation`)) true))

(fn `ResetHealthbar`
  (bind _ac_healthmanagement (`self.AC_Healthmanagement`))
  (cast `/Game/06_UI/WB_EnemyHealthbar` (`WidgetComponent.GetUserWidgetObject` (`self.Healthbar`)))
  (`SceneComponent.SetVisibility` (`self.Healthbar`) false false)
  (set `/Game/99_Testarea/TonyTeststuff/AC_Healthmanagement.CurrentHealth` (`/Game/99_Testarea/TonyTeststuff/AC_Healthmanagement.MaxHealth` _ac_healthmanagement) _ac_healthmanagement))

(fn `SetCollision`
  (params (EnableOrDisable :type Boolean))
  (if EnableOrDisable
    (`PrimitiveComponent.SetCollisionEnabled` (`self.Aura`) "QueryOnly")
    (`PrimitiveComponent.SetCollisionEnabled` (`self.CapsuleComponent`) "QueryAndPhysics")
    (`PrimitiveComponent.SetCollisionEnabled` (`self.Mesh`) "QueryAndPhysics")
    (else
      (`PrimitiveComponent.SetCollisionEnabled` (`self.Aura`) "NoCollision")
      (`PrimitiveComponent.SetCollisionEnabled` (`self.CapsuleComponent`) "NoCollision")
      (`PrimitiveComponent.SetCollisionEnabled` (`self.Mesh`) "NoCollision"))))

(fn `SetPath`
  (params (path :type "/Game/99_Testarea/Markus/EnemyPathing/ST_Path Structure"))
  (bind _output_get (set `self.Path` path))
  (bind ((`PathParts_10_687F04E2456F2EE5AF5BE0B764942AB2` _pathparts) (`Index_11_D425B7364D02A7631BFDD480EC2CBEF2` _index)) (break `/Game/99_Testarea/Markus/EnemyPathing/ST_Path` _output_get))
  (bind _spline (`/Game/99_Testarea/Markus/EnemyPathing/BP_PathParts.Spline` (`|GetArrayItem` _pathparts _index)))
  (set `self.MaxSplineDistance` (`SplineComponent.GetSplineLength` _spline))
  (`self.Check Reverse Travel` _spline))

(fn `SetupEnemy`
  (`self.SpawnDefaultController`)
  (set `self.SaveMaxWalkSpeed` (`self.MoveSpeed`))
  (bind _returnvalue (`GameplayStatics.GetActorOfClass` "/Game/03_GameplayAssets/05_Portals/BP_EnemySpawnManager.BP_EnemySpawnManager_C"))
  (set `self.SpawnManager` _returnvalue)
  (bind _returnvalue_2 (`GameplayStatics.GetActorOfClass` "/MoveIt/Example/BP_MoveIt_ExampleCharacter.BP_MoveIt_ExampleCharacter_C"))
  (set `self.Player` _returnvalue_2)
  (bind _returnvalue_3 (`GameplayStatics.GetActorOfClass` "/Game/03_GameplayAssets/02_Nexus/BP_Nexus.BP_Nexus_C"))
  (set `self.Nexus` _returnvalue_3)
  (bind _returnvalue_4 (`GameplayStatics.GetActorOfClass` "/Game/06_UI/01_Cards/BP_CardManager.BP_CardManager_C"))
  (set `self.CardManager` _returnvalue_4)
  (`self.SetActorTickEnabled` false)
  (`ActorComponent.SetComponentTickEnabled` (`self.AC_Healthmanagement`) false))

(fn `StartDogePath`
  (params (path :type "SplineComponent Object Reference") (setBy :type "Actor Object Reference"))
  (if (not (== setBy (`self.DogePathSetBy`)))
    (set `self.DogePathSetBy` setBy)
    (bind _output_get (set `self.DogeSpline` path))
    (set `self.ReverseTravelSave` (`self.ReverseTravel`))
    (set `self.DistanceAlongSpline` 0.0)
    (set `self.MaxSplineDistance` (`SplineComponent.GetSplineLength` _output_get))
    (`self.Check Reverse Travel` (`self.DogeSpline`))))

(fn `UpdateDistances`
  (params (DeltaTime :type "Float (double-precision)"))
  (bind _nexus (`self.Nexus`))
  (set `self.DamageDelayTimer` (- (`self.DamageDelayTimer`) DeltaTime))
  (`|ExecutionSequence`
    (:`then_0`
      (if (and (<= (`self.GetDistanceTo` (`self.Player`)) (`self.AuraRadius`)) (< (`self.DamageDelayTimer`) 0.0))
        (set `self.DamageDelayTimer` (`self.DamageDelay`))
        (`/Game/99_Testarea/TonyTeststuff/AC_Healthmanagement.TakeDamage` (`/MoveIt/Example/BP_MoveIt_ExampleCharacter.AC_Healthmanagement` (`self.Player`)) (`self.Damage`))))
    (:`then_1`
      (if (<= (- (`self.GetDistanceTo` _nexus) (`/Game/03_GameplayAssets/02_Nexus/BP_Nexus.NexusRadius` _nexus)) (`self.AuraRadius`))
        (`/Game/99_Testarea/TonyTeststuff/AC_Healthmanagement.TakeDamage` (`/Game/03_GameplayAssets/02_Nexus/BP_Nexus.AC_Healthmanagement` (`self.Nexus`)) (`self.Damage`))
        (`self.DYINGFunction` true)))))

(fn `UpdateHealthbar`
  (bind _aswb_enemy_healthbar (cast `/Game/06_UI/WB_EnemyHealthbar` (`WidgetComponent.GetUserWidgetObject` (`self.Healthbar`))))
  (set `/Game/06_UI/WB_EnemyHealthbar.CurrentHealth` (/ (`/Game/99_Testarea/TonyTeststuff/AC_Healthmanagement.CurrentHealth` (`self.AC_Healthmanagement`)) (`/Game/99_Testarea/TonyTeststuff/AC_Healthmanagement.MaxHealth` (`self.AC_Healthmanagement`))) _aswb_enemy_healthbar))

(fn `UserConstructionScript`)