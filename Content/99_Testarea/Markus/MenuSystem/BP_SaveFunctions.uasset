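; BP_SaveFunctions provides helper functions for loading and saving the game's BP_SaveGame object in a single fixed save slot.
; LoadSaveGame loads the slot and casts it to BP_SaveGame, creating and immediately saving a new object if that fails, then returns the result.
; SaveGame writes a passed-in save object back to the same slot.
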(fn `LoadSaveGame`
  (returns (saveObject :type "/Game/99_Testarea/Markus/MenuSystem/BP_SaveGame Object Reference"))
  (locals (loadedSave :type "/Game/99_Testarea/Markus/MenuSystem/BP_SaveGame Object Reference"))
  (bind _returnvalue (`GameplayStatics.LoadGameFromSlot` "save"))
  (bind (_asbp_save_game _bsuccess) (cast `/Game/99_Testarea/Markus/MenuSystem/BP_SaveGame` _returnvalue :!pure true))
  (if _bsuccess
    (set `local.loadedSave` _asbp_save_game)
    (else
      (bind _returnvalue_2 (`GameplayStatics.CreateSaveGameObject` "/Game/99_Testarea/Markus/MenuSystem/BP_SaveGame.BP_SaveGame_C"))
      (bind _output_get (set `local.loadedSave` _returnvalue_2))
      (`GameplayStatics.SaveGameToSlot` _output_get "save")))
  (return (`local.loadedSave`)))

(fn `SaveGame`
  (params (save :type "/Game/99_Testarea/Markus/MenuSystem/BP_SaveGame Object Reference"))
  (`GameplayStatics.SaveGameToSlot` save "save"))