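; BP_AuraTower is a tower Blueprint that hits every enemy in range at once, as an aura.
; Its SpawnProjectile function looks up projectile data by ProjectileID, then applies it and plays an impact effect on each actor in EnemiesInRange.
; No projectile actor is spawned in this graph.
; Tick and construction only call the parent, and range tracking is not defined here.
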(event `self.ReceiveTick`
  (params (DeltaSeconds :type "Float (single-precision)"))
  (`parent.ReceiveTick` DeltaSeconds))

(fn `SpawnProjectile`
  (locals (HitActor :type "Actor Object Reference") (HealthManager :type "/Game/99_Testarea/TonyTeststuff/AC_Healthmanagement Object Reference") (ProjectileData :type "/Game/99_Testarea/Markus/ProjectileData/ST_Projectiles Structure"))
  (bind _projectiledata (`/Game/99_Testarea/Markus/ProjectileData/BP_ProjectileDataHandle.GetProjectileData` (`self.Projectile ID`)))
  (set `local.ProjectileData` _projectiledata)
  (for _array_element (`self.EnemiesInRange`)
    (`/Game/99_Testarea/Markus/ProjectileData/BP_ProjectileDataHandle.HandleProjectileData` (`local.ProjectileData`) _array_element)
    (`/Game/99_Testarea/Markus/ProjectileData/BP_ProjectileDataHandle.PlayImpactEffectAtActorPosition` (`local.ProjectileData`) _array_element)))

(fn `UserConstructionScript`
  (`parent.UserConstructionScript`))