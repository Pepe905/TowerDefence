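; BP_EliteEnemyTest is an elite enemy subclass that fires projectiles at the player when in range.
; Tick runs a shot timer and distance check, spawning a projectile rotated toward the player.
; Death drops a card and reports points to BP_PointSystem unless self-destructed, then always despawns.
; Despawning notifies SpawnManager, grants Nexus mana, resets health and parks the actor below the level with collision and ticking off rather than destroying it.
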(event `self.ReceiveBeginPlay`
  (set `self.Damage` 50.0))

(event `self.ReceiveTick`
  (params (DeltaSeconds :type "Float (single-precision)"))
  (`parent.ReceiveTick` DeltaSeconds)
  (`self.LookoutForPlayer` DeltaSeconds))

(event `/Game/99_Testarea/TonyTeststuff/BPI_ActorStateChange.Death`
  (params (selfDescruct :type Boolean))
  (`KismetSystemLibrary.PrintString` "calledsubClass")
  (if (not selfDescruct)
    (`self.DropCard`)
    (bind _returnvalue (`GameplayStatics.GetActorOfClass` "/Game/99_Testarea/Markus/PointSystem/BP_PointSystem.BP_PointSystem_C"))
    (`/Game/99_Testarea/Markus/PointSystem/BP_PointSystem.EnemyDeath` _returnvalue (`self.Points`)))
  (`self.DespawnEliteEnemy`))

(fn `DespawnEliteEnemy`
  (`/Game/03_GameplayAssets/05_Portals/BP_EnemySpawnManager.DespawnEnemies` (`self.SpawnManager`) self)
  (`self.SetCollision` false)
  (`/Game/03_GameplayAssets/05_Portals/BP_EnemySpawnManager.CheckEnemiesLeft` (`self.SpawnManager`))
  (`/Game/03_GameplayAssets/02_Nexus/BP_Nexus.ManaGain` (`self.Nexus`) (`self.Mana Increase`))
  (`self.K2_AddActorWorldOffset` (0.0 0.0 -1000.0) false true)
  (`self.ResetHealthbar`)
  (`self.SetActorTickEnabled` false)
  (`ActorComponent.SetComponentTickEnabled` (`self.AC_Healthmanagement`) false))

(fn `LookoutForPlayer`
  (params (DeltaSeconds :type "Float (double-precision)"))
  (locals (Enemy :type "/Game/04_Characters/02_Enemies/BP_EnemyTest Object Reference"))
  (set `self.TimeSinceLastShot` (+ DeltaSeconds (`self.TimeSinceLastShot`)))
  (if (>= (`self.TimeSinceLastShot`) (`self.TimeBetweenShots`))
    (if (< (`self.GetDistanceTo` (`self.Player`)) (`self.LookOutRange`))
      (`self.ShootAtPlayer`))))

(fn `ShootAtPlayer`
  (bind _returnvalue (`self.K2_GetActorLocation` self))
  (set `self.TimeSinceLastShot` 0.0)
  (bind _returnvalue_2 (`|SpawnActorFromClass` "/Game/99_Testarea/Pepe/Projectile.Projectile_C" (`KismetMathLibrary.MakeTransform` _returnvalue (`KismetMathLibrary.FindLookAtRotation` _returnvalue (`SceneComponent.K2_GetComponentLocation` (`Actor.RootComponent` (`self.Player`))))) "Undefined" "OverrideRootScale" null null))
  (`/Game/99_Testarea/Pepe/Projectile.SetInit` _returnvalue_2 (`self.ProjectileID`) "ECC_GameTraceChannel2" "ECR_Overlap"))

(fn `UserConstructionScript`
  (`parent.UserConstructionScript`))