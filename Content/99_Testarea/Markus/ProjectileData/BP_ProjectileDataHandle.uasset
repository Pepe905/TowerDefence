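; Shared projectile helper that looks up stats in DT_Projectiles by ID and applies hit effects to actors.
; HandleProjectileData feeds damage and tick damage to the target's AC_Healthmanagement and sends it a slowdown message, with debug prints.
; PlayImpactEffectAtActorPosition spawns the row's Niagara impact effect at the hit actor.
; CheckArea returns sphere-overlapped actors, querying Pawns or a custom object type based on the collision sphere's channel response.
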(fn `CheckArea`
  (params (hitPosition :type "Vector Structure") (collisonSphere :type "StaticMeshComponent Object Reference") (checkRadius :type "Float (double-precision)") (IgnoreActors :type "Array of Actor Object Reference"))
  (returns (hitActors :type "Array of Actor Object Reference"))
  (locals (TypeCollisionCheck :type "Array of EObjectTypeQuery Enum") (ProjectileData :type "/Game/99_Testarea/Markus/ProjectileData/ST_Projectiles Structure") (radius :type "Float (double-precision)"))
  (set `local.radius` checkRadius)
  (if (`|EnumEquality` (`PrimitiveComponent.GetCollisionResponseToChannel` collisonSphere "ECC_GameTraceChannel2") "ECR_Ignore")
    (set `local.TypeCollisionCheck` (`|MakeArray` "ObjectTypeQuery9" :!type "EObjectTypeQuery Enum"))
    (else
      (set `local.TypeCollisionCheck` (`|MakeArray` "ObjectTypeQuery3" :!type "EObjectTypeQuery Enum"))))
  (bind _outactors (`KismetSystemLibrary.SphereOverlapActors` null hitPosition (`local.radius`) (`local.TypeCollisionCheck`) null IgnoreActors))
  (return _outactors))

(fn `GetProjectileData`
  (params (ProjectileID :type Name))
  (returns (ProjectileData :type "/Game/99_Testarea/Markus/ProjectileData/ST_Projectiles Structure"))
  (bind _returnvalue (`|GetDataTableRow` "/Game/99_Testarea/Markus/ProjectileData/DT_Projectiles.DT_Projectiles" ProjectileID)
    (:`then`
      (return _returnvalue))))

(fn `HandleProjectileData`
  (params (ProjectileData :type "/Game/99_Testarea/Markus/ProjectileData/ST_Projectiles Structure (by ref)") (HitActor :type "Actor Object Reference"))
  (locals (LocalProjectileData :type "/Game/99_Testarea/Markus/ProjectileData/ST_Projectiles Structure") (localHitActor :type "Actor Object Reference") (hitHealthManager :type "/Game/99_Testarea/TonyTeststuff/AC_Healthmanagement Object Reference"))
  (bind ((`Damage_101_B3C4CC01405E50C27ECACC8A6F8D0631` _damage) (`ChainCount_82_51C935DD478598FFDC57699A6DEB1846` _chaincount) (`TickDamage_102_A82A3F44484D6272458FBD80051A480A` _tickdamage) (`TickDamageCounter_99_17A4C6A24E5F9ECE79C10D85E9B3CCE7` _tickdamagecounter) (`TickDamageIntervall_96_584300894D71F1CA3E82CD9988BD18C8` _tickdamageintervall) (`Slowdown_93_C4CE1F2A43F1569DB8BAB89007CF883C` _slowdown) (`SlowdownDuration_94_BC26B9FF4015B0C66A4835B319D12E77` _slowdownduration)) (break `/Game/99_Testarea/Markus/ProjectileData/ST_Projectiles` ProjectileData))
  (bind _returnvalue (`Actor.GetComponentByClass` HitActor "/Game/99_Testarea/TonyTeststuff/AC_Healthmanagement.AC_Healthmanagement_C"))
  (`/Engine/EditorBlueprintResources/StandardMacros.IsValid` _returnvalue
    (:`Is Valid`
      (set `local.hitHealthManager` _returnvalue)
      (set `local.localHitActor` HitActor)
      (`/Game/99_Testarea/TonyTeststuff/AC_Healthmanagement.AddTickDamage` (`local.hitHealthManager`) _tickdamage _tickdamagecounter _tickdamageintervall)
      (message `/Game/99_Testarea/TonyTeststuff/BPI_ActorStateChange.SlowDown` (`local.localHitActor`) _slowdown _slowdownduration)
      (`/Game/99_Testarea/TonyTeststuff/AC_Healthmanagement.TakeDamage` (`local.hitHealthManager`) _damage)
      (`KismetSystemLibrary.PrintString` null (`KismetStringLibrary.Conv_DoubleToString` (`.Slowdown_93_C4CE1F2A43F1569DB8BAB89007CF883C` (break `/Game/99_Testarea/Markus/ProjectileData/ST_Projectiles` ProjectileData))) true true (struct :`R` 1.0 :`B` 0.846875 :`A` 1.0)))
    (:`Is Not Valid`
      (`KismetSystemLibrary.PrintString` null "NO AC HEALTHMANAGEMENT"))))

(fn `PlayImpactEffectAtActorPosition`
  (params (ProjectileData :type "/Game/99_Testarea/Markus/ProjectileData/ST_Projectiles Structure (by ref)") (HitActor :type "Actor Object Reference"))
  (bind (_projectilename _range _speed _scale _impactarea _damage _chaincount _tickdamage _tickdamagecounter _tickdamageintervall _slowdown _slowdownduration _stunduration _sm_mesh_projectileoptics _m_texture _ns_launch_vfx _ns_flight_vfx _ns_impact_vxf) (break `/Game/99_Testarea/Markus/ProjectileData/ST_Projectiles` ProjectileData))
  (bind (_returnvalue_location _returnvalue_rotation) (`KismetMathLibrary.BreakTransform` (`Actor.GetTransform` HitActor)))
  (`/Engine/EditorBlueprintResources/StandardMacros.IsValid` _ns_impact_vxf
    (:`Is Valid`
      (`NiagaraFunctionLibrary.SpawnSystemAtLocation` null _ns_impact_vxf _returnvalue_location _returnvalue_rotation (0.1 0.1 0.1)))))