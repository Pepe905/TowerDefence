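; Enemy pathing helper functions that operate on a path struct made of ordered spline parts.
; CheckIsBlocked advances a blocked path's BlockedIndex past freed parts, stopping at the first blocked one or marking the path free after the last.
; CheckSplineDistance carries excess travel distance into following parts, updating the path index by reference and returning the adjusted distance, current spline length and a change flag.
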(fn `Check Spline Distance`
  (params (inputPath :type "/Game/99_Testarea/Markus/EnemyPathing/ST_Path Structure (by ref)") (inputDistanceAlongSpline :type "Float (double-precision)") (maxSplineDistance :type "Float (double-precision)"))
  (returns (outDistanceAlongSpline :type "Float (double-precision)") (outMaxSplineDistance :type "Float (double-precision)") (change :type Boolean))
  (locals (path :type "/Game/99_Testarea/Markus/EnemyPathing/ST_Path Structure") (distanceAlongSpline :type "Float (double-precision)") (maxDistance :type "Float (double-precision)") (changed :type Boolean))
  (bind _path (`local.path`))
  (bind (_pathparts _index) (break `/Game/99_Testarea/Markus/EnemyPathing/ST_Path` (`local.path`)))
  (set `local.path` inputPath)
  (set `local.distanceAlongSpline` inputDistanceAlongSpline)
  (set `local.maxDistance` maxSplineDistance)
  (while (and (> (`local.distanceAlongSpline`) (`local.maxDistance`)) (< _index (`KismetArrayLibrary.Array_Length` _pathparts)))
    (set `local.distanceAlongSpline` (- (`local.distanceAlongSpline`) (`local.maxDistance`)))
    (bind _structout (setmembers `/Game/99_Testarea/Markus/EnemyPathing/ST_Path` :`StructRef` _path :`Index` (+ (`.Index_11_D425B7364D02A7631BFDD480EC2CBEF2` (break `/Game/99_Testarea/Markus/EnemyPathing/ST_Path` _path)) 1)))
    (bind ((`PathParts_10_687F04E2456F2EE5AF5BE0B764942AB2` _pathparts_2) (`Index_11_D425B7364D02A7631BFDD480EC2CBEF2` _index_2)) (break `/Game/99_Testarea/Markus/EnemyPathing/ST_Path` _structout))
    (set `local.maxDistance` (`SplineComponent.GetSplineLength` (`/Game/99_Testarea/Markus/EnemyPathing/BP_PathParts.Spline` (`|GetArrayItem` _pathparts_2 _index_2))))
    (set `local.changed` true))
  (`|VariableSetRef` inputPath (`local.path`))
  (return (`local.distanceAlongSpline`) (`local.maxDistance`) (`local.changed`)))

(fn `CheckIsBlocked`
  (params (path :type "/Game/99_Testarea/Markus/EnemyPathing/ST_Path Structure"))
  (returns (outPath :type "/Game/99_Testarea/Markus/EnemyPathing/ST_Path Structure"))
  (locals (break :type Boolean) (changePath :type "/Game/99_Testarea/Markus/EnemyPathing/ST_Path Structure"))
  (bind _changepath (`local.changePath`))
  (bind _changepath_2 (`local.changePath`))
  (bind _output_get (set `local.changePath` path))
  (bind ((`PathParts_10_687F04E2456F2EE5AF5BE0B764942AB2` _pathparts) (`BlockedIndex_12_D18DD651417607449B8150A8FD72BF65` _blockedindex) (`IsFree_8_E28C161941444E240D38F3B26AC8EF44` _isfree)) (break `/Game/99_Testarea/Markus/EnemyPathing/ST_Path` _output_get))
  (if (not _isfree)
    (while (`KismetMathLibrary.BooleanNOR` _isfree (`local.break`))
      (if (`/Game/99_Testarea/Markus/EnemyPathing/BP_PathParts.IsFree` (`|GetArrayItem` _pathparts _blockedindex))
        (setmembers `/Game/99_Testarea/Markus/EnemyPathing/ST_Path` :`StructRef` _changepath :`BlockedIndex` (+ (`.BlockedIndex_12_D18DD651417607449B8150A8FD72BF65` (break `/Game/99_Testarea/Markus/EnemyPathing/ST_Path` _changepath)) 1))
        (bind _isfree_2 (`self.CheckLastBlockedReached` _changepath_2))
        (setmembers `/Game/99_Testarea/Markus/EnemyPathing/ST_Path` :`StructRef` _changepath_2 :`IsFree` _isfree_2)
        (else
          (set `local.break` true))))
    (return (`local.changePath`))))

(fn `CheckLastBlockedReached`
  (params (path :type "/Game/99_Testarea/Markus/EnemyPathing/ST_Path Structure"))
  (returns (IsFree :type Boolean))
  (locals (free :type Boolean :default false))
  (bind ((`PathParts_10_687F04E2456F2EE5AF5BE0B764942AB2` _pathparts) (`BlockedIndex_12_D18DD651417607449B8150A8FD72BF65` _blockedindex)) (break `/Game/99_Testarea/Markus/EnemyPathing/ST_Path` path))
  (return (>= _blockedindex (`KismetArrayLibrary.Array_Length` _pathparts))))