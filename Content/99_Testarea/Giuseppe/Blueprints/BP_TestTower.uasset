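; Test defensive statue tower that shoots projectiles at nearby BP_EnemyTest actors, with a glow that signals aggression at night.
; Each tick, a sphere overlap and visibility traces pick a target, favouring the closest in sight.
; During the night phase, a dynamic material interpolates between night and aggressive colours based on enemies in range, setting TowerIsRed.
; That flag gates cooldown-timed firing from WeaponSocket; the night-to-day colour change is left unwired.
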(event `ChangeTowerColor`
  (params (A :type "/Game/99_Testarea/Markus/EDayState Enum" :default "NewEnumerator0"))
  (set `self.Current Phase` A)
  (`self.DNCycleStatueGlow` A)
  (set `self.ColourEnemyInSight` false))

(event `self.ReceiveBeginPlay`
  (`KismetArrayLibrary.Array_Clear` (`self.EnemiesInRange`))
  (`PrimitiveComponent.SetMaterial` (`self.SM_Tower`) 1 (`self.TowerGlowMatInst`))
  (bind _output_get (set `self.EmissiveColor` (`self.EmissiveColorDay`)))
  (`MaterialInstanceDynamic.SetVectorParameterValue` (`self.TowerGlowMatInst`) "EmissiveColor" _output_get))

(event `self.ReceiveTick`
  (params (DeltaSeconds :type "Float (single-precision)"))
  (set `self.Delta Seconds` DeltaSeconds)
  (`self.FindBestTarget`)
  (`self.Target`
    (:`then`
      (`self.EnemyStatueGlow`)
      (`self.DelayFire` DeltaSeconds))
    (:`else`
      (if (`KismetArrayLibrary.Array_IsEmpty` (`self.EnemiesInRange`))
        (set `self.ColourEnemyInSight` false)
        (`self.EnemyStatueGlow`)))))

(event `DayToNight`
  ;[1 1 1] DayToNight
  (bind _returnvalue (`MaterialInstanceDynamic.K2_GetVectorParameterValue` (`self.TowerGlowMatInst`) "EmissiveColor"))
  (`MaterialInstanceDynamic.SetVectorParameterValue` :`self` (`self.TowerGlowMatInst`) :`ParameterName` "EmissiveColor"))

(event `GlowOnEnemy`
  ;[1 1 1] FriendlyToAgressive
  (bind _returnvalue (`MaterialInstanceDynamic.K2_GetVectorParameterValue` (`self.TowerGlowMatInst`) "EmissiveColor"))
  (`MaterialInstanceDynamic.SetVectorParameterValue` (`self.TowerGlowMatInst`) "EmissiveColor" (`KismetMathLibrary.CInterpTo` _returnvalue (`self.EmissiveColorAggressive`) (`self.Delta Seconds`) 6.5))
  (set `self.TowerIsRed` true))

(event `GlowAfterNoEnemy`
  ;[1 1 1] AgressiveToFriendly
  (bind _returnvalue (`MaterialInstanceDynamic.K2_GetVectorParameterValue` (`self.TowerGlowMatInst`) "EmissiveColor"))
  (`MaterialInstanceDynamic.SetVectorParameterValue` (`self.TowerGlowMatInst`) "EmissiveColor" (`KismetMathLibrary.CInterpTo` _returnvalue (`self.EmissiveColorNight`) (`self.Delta Seconds`) 6.5))
  (set `self.TowerIsRed` false))

(event `NightToDay`
  ;[1 1 1] NightToDay
  (bind _returnvalue (`MaterialInstanceDynamic.K2_GetVectorParameterValue` (`self.TowerGlowMatInst`) "EmissiveColor")))

(fn `AnyEnemiesLeft`
  (returns (ReturnValue :type Boolean))
  (return (not (`KismetArrayLibrary.Array_IsEmpty` (`self.EnemiesInRange`)))))

(fn `CreateMaterialInstance`
  (params (EmissiveColor :type "LinearColor Structure"))
  (returns (ReturnValue :type "MaterialInstanceDynamic Object Reference"))
  (bind _returnvalue (`KismetMaterialLibrary.CreateDynamicMaterialInstance` "/Game/99_Testarea/Giuseppe/Materials/MI_Statue_KnightTest.MI_Statue_KnightTest"))
  (`MaterialInstanceDynamic.SetVectorParameterValue` _returnvalue "EmissiveColor" EmissiveColor)
  (return _returnvalue))

(fn `DelayFire`
  (params (deltaTime :type "Float (double-precision)"))
  (set `self.Time` (+ deltaTime (`self.Time`)))
  (if (>= (`self.Time`) (`self.TimeBetweenShots`))
    (set `self.Time` (- (`self.Time`) (`self.TimeBetweenShots`)))
    (if (`self.TowerIsRed`)
      (`self.FireEnemy`)
      (else
        (`KismetSystemLibrary.PrintString` "Cannot shoot, Color not red")))))

(fn `DNCycleStatueGlow`
  (params (A :type "/Game/99_Testarea/Markus/EDayState Enum" :default "NewEnumerator0"))
  (if (or (`|EnumEquality` A "NewEnumerator0") (`|EnumEquality` A "NewEnumerator2"))
    (`self.NightToDay`)
    (elif (`|EnumEquality` A "NewEnumerator1")
      (`self.DayToNight`))))

(fn `EnemyStatueGlow`
  (if (`|EnumEquality` (`self.Current Phase`) "NewEnumerator1")
    (bind _returnvalue (`self.AnyEnemiesLeft`))
    (if _returnvalue
      (`self.GlowOnEnemy`)
      (else
        (`self.GlowAfterNoEnemy`)))))

(fn `FindBestTarget`
  (locals (BestDistance :type "Float (double-precision)") (CurrentDistance :type "Float (double-precision)") (BestTarget :type "Actor Object Reference") (CurrentTarget :type "Actor Object Reference"))
  (set `local.BestDistance` (+ (`self.SensingRange`) 1.0))
  (bind _outactors (`KismetSystemLibrary.SphereOverlapActors` (`self.K2_GetActorLocation`) (`self.SensingRange`) (`|MakeArray` "ObjectTypeQuery9" :!type "EObjectTypeQuery Enum") "/Game/04_Characters/02_Enemies/BP_EnemyTest.BP_EnemyTest_C"))
  (bind _output_get (set `self.EnemiesInRange` _outactors))
  (for _array_element _output_get
    (bind _output_get_2 (set `local.CurrentTarget` _array_element))
    (bind _output_get_3 (set `local.CurrentDistance` (`self.GetDistanceTo` _output_get_2 self)))
    (if (or (< _output_get_3 (`local.BestDistance`)) (not (`KismetSystemLibrary.IsValid` (`local.BestTarget`))))
      (bind _result (`self.HasLineOfSight` (`SceneComponent.K2_GetComponentLocation` (`self.SM_Tower`)) (`self.K2_GetActorLocation` (`local.CurrentTarget`)) (`|MakeArray` self (`local.CurrentTarget`) :!type "Actor Object Reference")))
      (if _result
        (set `local.BestTarget` (`local.CurrentTarget`))
        (set `local.BestDistance` (`local.CurrentDistance`))
        (bind _output_get_4 (set `self.LockedOnTarget` _result))
        (set `self.ColourEnemyInSight` _output_get_4)
        (else
          (bind _returnvalue (`self.AnyEnemiesLeft`))
          (if _returnvalue
            (set `self.LockedOnTarget` false)
            (set `self.ColourEnemyInSight` false)
            (set `self.Target` null))))))
  (set `self.Target` (`local.BestTarget`)))

(fn `FireEnemy`
  (`self.SpawnProjectile`))

(fn `HasLineOfSight`
  (params (From :type "Vector Structure") (To :type "Vector Structure") (ActorsToIgnore :type "Array of Actor Object Reference (by ref)"))
  (returns (Result :type Boolean))
  (bind (_outhit _returnvalue) (`KismetSystemLibrary.LineTraceSingle` From To "TraceTypeQuery1" false ActorsToIgnore "ForDuration" false))
  (return (not _returnvalue)))

(fn `SpawnProjectile`
  (bind _target (`self.Target`))
  (bind _returnvalue (`SceneComponent.GetSocketLocation` (`self.SM_Tower`) "WeaponSocket"))
  (bind _returnvalue_location (`KismetMathLibrary.BreakTransform` (`SceneComponent.K2_GetComponentToWorld` (`Actor.RootComponent` _target))))
  (`/Engine/EditorBlueprintResources/StandardMacros.IsValid` _target
    (:`Is Valid`
      (bind _returnvalue_2 (`|SpawnActorFromClass` "/Game/99_Testarea/Pepe/Projectile.Projectile_C" (`KismetMathLibrary.MakeTransform` _returnvalue (`KismetMathLibrary.FindLookAtRotation` _returnvalue _returnvalue_location) (0.1 0.1 0.1)) "Undefined" "OverrideRootScale" null null))
      (`/Game/99_Testarea/Pepe/Projectile.SetInit` _returnvalue_2 "0")
      (`PrimitiveComponent.SetCollisionResponseToChannel` (`/Game/99_Testarea/Pepe/Projectile.Sphere` _returnvalue_2) "ECC_GameTraceChannel2" "ECR_Ignore")
      (`KismetSystemLibrary.PrintString` "I am Shooting"))))

(fn `UserConstructionScript`
  (bind _returnvalue (`self.CreateMaterialInstance` (`self.EmissiveColor`)))
  (set `self.TowerGlowMatInst` _returnvalue))