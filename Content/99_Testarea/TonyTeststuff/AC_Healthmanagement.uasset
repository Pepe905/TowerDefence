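; Actor component that manages its owner's health, with instant and damage-over-time hits.
; TakeDamage lowers CurrentHealth, sends DmgTakenMessage to the owner, then sends DeathMessage when health reaches zero or below.
; AddTickDamage queues struct entries that Tick advances by delta time, applying damage each interval and iterating in reverse to remove expired ones safely.
; MaxHealth is captured from CurrentHealth at BeginPlay, and HealDamage is an empty stub.
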(event `self.ReceiveBeginPlay`
  (set `self.MaxHealth` (`self.CurrentHealth`)))

(event `self.ReceiveTick`
  (params (DeltaSeconds :type "Float (single-precision)"))
  (`self.TickDamageUpdate` DeltaSeconds))

(fn `AddTickDamage`
  (params (TickDamage :type "Float (double-precision)") (TickCounter :type Integer) (TickIntervall :type "Float (double-precision)"))
  (if (not (<= TickCounter 0))
    (`KismetArrayLibrary.Array_Add` (`self.TickObject`) (make `/Game/99_Testarea/Markus/ProjectileData/ST_TickObject` TickDamage TickCounter TickIntervall))))

(fn `CheckHealth`
  (if (not (> (`self.CurrentHealth`) 0.0))
    (message `/Game/99_Testarea/TonyTeststuff/BPI_ActorStateChange.Death` (`self.GetOwner` self) false)))

(fn `HealDamage`)

(fn `TakeDamage`
  (params (Damage :type "Float (double-precision)"))
  (set `self.CurrentHealth` (- (`self.CurrentHealth`) Damage))
  (message `/Game/99_Testarea/TonyTeststuff/BPI_ActorStateChange.DmgTaken` (`self.GetOwner` self))
  (`self.CheckHealth`))

(fn `TickDamageUpdate`
  (params (DeltaTime :type "Float (double-precision)"))
  (locals (CurrentTickObject :type "/Game/99_Testarea/Markus/ProjectileData/ST_TickObject Structure") (CurrentIndex :type Integer))
  (bind (_arrayindex _arrayelement) (`/Engine/EditorBlueprintResources/StandardMacros.ReverseForEachLoop` (`self.TickObject`))
    (:`LoopBody`
      (set `local.CurrentIndex` _arrayindex)
      (bind _output_get (set `local.CurrentTickObject` _arrayelement))
      (if (<= (`.TickCounter_9_5AF5EEDF49DA514D0A71B5ADDB0A1496` (break `/Game/99_Testarea/Markus/ProjectileData/ST_TickObject` _output_get)) 0)
        (`KismetArrayLibrary.Array_Remove` (`self.TickObject`) (`local.CurrentIndex`))
        (else
          (bind _structout (setmembers `/Game/99_Testarea/Markus/ProjectileData/ST_TickObject` :`StructRef` (`local.CurrentTickObject`) :`TickStartTime` (+ (`.TickStartTime_12_AA491A474FC8EA7495545FA058711D03` (break `/Game/99_Testarea/Markus/ProjectileData/ST_TickObject` _output_get)) DeltaTime)))
          (if (> (`.TickStartTime_12_AA491A474FC8EA7495545FA058711D03` (break `/Game/99_Testarea/Markus/ProjectileData/ST_TickObject` _structout)) (`.TickIntervall_6_DBA62502493FD5BAB2F166874988845F` (break `/Game/99_Testarea/Markus/ProjectileData/ST_TickObject` _structout)))
            (bind _structout_2 (setmembers `/Game/99_Testarea/Markus/ProjectileData/ST_TickObject` :`StructRef` (`local.CurrentTickObject`) :`TickCounter` (- (`.TickCounter_9_5AF5EEDF49DA514D0A71B5ADDB0A1496` (break `/Game/99_Testarea/Markus/ProjectileData/ST_TickObject` _structout)) 1) :`TickStartTime` 0.0))
            (`self.TakeDamage` (break `/Game/99_Testarea/Markus/ProjectileData/ST_TickObject` _structout_2)))
          (`KismetArrayLibrary.Array_Set` (`self.TickObject`) (`local.CurrentIndex`) (`local.CurrentTickObject`)))))))