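; BP_PointSystem is an actor that keeps the player's score, kill count and play time.
; On BeginPlay it registers itself with the example character and its demo widget, with tick off until StartPointSystem runs.
; While ticking, points drain over time and the killing spree timer counts down.
; Kills award points times a growing spree multiplier; player or Nexus hits subtract points and reset the spree.
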(event `self.ReceiveBeginPlay`
  (`self.SetActorTickEnabled` false)
  (bind _returnvalue (`GameplayStatics.GetActorOfClass` "/MoveIt/Example/BP_MoveIt_ExampleCharacter.BP_MoveIt_ExampleCharacter_C"))
  (set `/MoveIt/Example/BP_MoveIt_ExampleCharacter.PointSystem` self _returnvalue)
  (set `/Game/06_UI/WB_HUD.PointSystem` self (`/MoveIt/Example/BP_MoveIt_ExampleCharacter.DemoWidget` _returnvalue))
  (set `self.IntCurrentPoints` (`KismetMathLibrary.FTrunc` (`self.CurrentPoints`))))

(event `self.ReceiveTick`
  (params (DeltaSeconds :type "Float (single-precision)"))
  (set `self.PlayTimeInSeconds` (+ DeltaSeconds (`self.PlayTimeInSeconds`)))
  (`self.UpdatePoints` DeltaSeconds)
  (`self.UpdateKillingSpree` DeltaSeconds)
  (set `self.IntCurrentPoints` (`KismetMathLibrary.FTrunc` (`self.CurrentPoints`))))

(fn `EnemyDeath`
  (params (points :type "Float (double-precision)"))
  (`/Engine/EditorBlueprintResources/StandardMacros.IncrementInt` (`self.EnemyKillCounter`)
    (:`  `
      (`/Engine/EditorBlueprintResources/StandardMacros.IncrementFloat` (`self.KillingSpreeMultiplicator`)
        (:`  `
          (set `self.KillingSpreeTimer` (`self.KillingSpreeBaseTime`))
          (set `self.CurrentPoints` (+ (* points (`self.KillingSpreeMultiplicator`)) (`self.CurrentPoints`))))))))

(fn `NexusTakeDmg`
  (`self.ResetKillingSpree`)
  (set `self.CurrentPoints` (- (`self.CurrentPoints`) (`self.NexusHitPointReduction`))))

(fn `PlayerTakeDmg`
  (`self.ResetKillingSpree`)
  (set `self.CurrentPoints` (- (`self.CurrentPoints`) (`self.PlayerHitPointReduction`))))

(fn `ResetKillingSpree`
  (set `self.KillingSpreeMultiplicator` 1.0)
  (set `self.KillingSpreeTimer` 0.0))

(fn `StartPointSystem`
  (`self.SetActorTickEnabled` true))

(fn `StopPointSystem`
  (`self.SetActorTickEnabled` false))

(fn `UpdateKillingSpree`
  (params (deltaTime :type "Float (double-precision)"))
  (if (> (`self.KillingSpreeTimer`) 0.0)
    (bind _output_get (set `self.KillingSpreeTimer` (- (`self.KillingSpreeTimer`) deltaTime)))
    (if (<= _output_get 0.0)
      (`self.ResetKillingSpree`))))

(fn `UpdatePoints`
  (params (deltTime :type "Float (double-precision)"))
  (set `self.CurrentPoints` (- (`self.CurrentPoints`) (* deltTime (`self.PointReductionPerSecond`)))))

(fn `UserConstructionScript`)